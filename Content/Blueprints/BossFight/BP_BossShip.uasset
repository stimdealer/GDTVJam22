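; Boss ship for the boss fight, with armor, shield, turret and cannon stats set by game-instance difficulty.
; A detection sphere stores the player ship as the turret target.
; Tick timers drive a charged beam cannon, damaging players inside CannonBox after a delay, and four-missile volleys aimed at the player, retrying until that reference is valid.
; Death destroys the ship and notifies the warp gate.
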(event `self.ReceiveBeginPlay`
  (bind _missilelocations (`self.MissileLocations`))
  (bind _turrets (`self.Turrets`))
  (`|ExecutionSequence`
    (:`then_0`
      (`KismetArrayLibrary.Array_Add` _turrets (`self.CenterTurret_A`))
      (`KismetArrayLibrary.Array_Add` _turrets (`self.CenterTurret_B`))
      (`KismetArrayLibrary.Array_Add` _turrets (`self.StbdTurret_A`))
      (`KismetArrayLibrary.Array_Add` _turrets (`self.StbdTurret_B`))
      (`KismetArrayLibrary.Array_Add` _turrets (`self.PortTurret_A`))
      (`KismetArrayLibrary.Array_Add` _turrets (`self.PortTurret_B`))
      (`self.SetBossStats`))
    (:`then_1`
      (`KismetArrayLibrary.Array_Add` _missilelocations (`SceneComponent.K2_GetComponentLocation` (`self.MissileSpawn_1`)))
      (`KismetArrayLibrary.Array_Add` _missilelocations (`SceneComponent.K2_GetComponentLocation` (`self.MissileSpawn_2`)))
      (`KismetArrayLibrary.Array_Add` _missilelocations (`SceneComponent.K2_GetComponentLocation` (`self.MissileSpawn_3`)))
      (`KismetArrayLibrary.Array_Add` _missilelocations (`SceneComponent.K2_GetComponentLocation` (`self.MissileSpawn_4`))))))

(event `self.ReceiveTick`
  (params (DeltaSeconds :type "Float (single-precision)"))
  (`self.MainCannonChargeUp` DeltaSeconds)
  (`self.MissileVolley` DeltaSeconds)
  (`KismetSystemLibrary.PrintString` (`KismetStringLibrary.Conv_DoubleToString` (`self.CurrentArmor`)) true false (struct :`B` 1.0 :`A` 1.0) 0.0)
  (`KismetSystemLibrary.PrintString` (`KismetStringLibrary.Conv_DoubleToString` (`self.CurrentShield`)) true false (struct :`G` 1.0 :`A` 1.0) 0.0))

(event `self.UpdateStats`
  (params (InArmorPercent :type "Float (single-precision)") (InShieldPercent :type "Float (single-precision)"))
  (bind _aswbp_enemy_bars (cast `/Game/UI/WBP_EnemyBars` (`WidgetComponent.GetWidget` (`self.StatusBars`))))
  (`/Game/UI/WBP_EnemyBars.SetStats` _aswbp_enemy_bars InArmorPercent InShieldPercent))

(event `MainCannonFireEvent`
  (`self.MainCannonFire`)
  (`KismetSystemLibrary.Delay` 2.5)
  (`self.MainCannonDealDamage`))

(event `MainCannonTell`
  (`SceneComponent.SetVisibility` (`self.MainCannonPreview`) true false)
  (`KismetSystemLibrary.Delay` 1.5)
  (`SceneComponent.SetVisibility` (`self.MainCannonPreview`) false false))

(event `self.ShipDeath`
  (`KismetSystemLibrary.PrintString` "Boss Destroyed!" true false (struct :`G` 0.66 :`B` 1.0 :`A` 1.0) 20.0)
  (`self.K2_DestroyActor`)
  (`/Game/Blueprints/Environment/BP_WarpGate.BossDeath` (`self.WarpGateRef`)))

(event `self.PlayerDetectionSphere.OnComponentBeginOverlap`
  (params (OverlappedComponent :type "PrimitiveComponent Object Reference") (OtherActor :type "Actor Object Reference") (OtherComp :type "PrimitiveComponent Object Reference") (OtherBodyIndex :type Integer) (bFromSweep :type Boolean) (SweepResult :type "HitResult Structure (by ref)"))
  (`KismetSystemLibrary.PrintString` "Player ship detected!" true false (struct :`R` 1.0 :`G` 1.0 :`B` 1.0 :`A` 1.0) 30.0)
  (bind _asbp_player_phoenix (cast `/Game/Blueprints/BP_PlayerPhoenix` OtherActor))
  (set `self.PlayerShipRef` _asbp_player_phoenix)
  (`self.SetPlayerShipTargets`))

(event `SpawnMissile`
  (bind _playershipref (`self.PlayerShipRef`))
  (bind _playershipref_2 (`self.PlayerShipRef`))
  (bind _playershipref_3 (`self.PlayerShipRef`))
  (bind _playershipref_4 (`self.PlayerShipRef`))
  (bind _returnvalue (`SceneComponent.K2_GetComponentLocation` (`self.MissileSpawn_4`)))
  (bind _returnvalue_2 (`SceneComponent.K2_GetComponentLocation` (`self.MissileSpawn_1`)))
  (bind _returnvalue_3 (`SceneComponent.K2_GetComponentLocation` (`self.MissileSpawn_2`)))
  (bind _returnvalue_4 (`SceneComponent.K2_GetComponentLocation` (`self.MissileSpawn_3`)))
  (`|ExecutionSequence`
    (:`then_0`
      (`/Engine/EditorBlueprintResources/StandardMacros.IsValid` _playershipref :!label _label
        (:`Is Valid`
          (`|SpawnActorFromClass` "/Game/Blueprints/BossFight/BP_BossMissile.BP_BossMissile_C" (`KismetMathLibrary.MakeTransform` _returnvalue_2 (`KismetMathLibrary.Conv_VectorToRotator` (`KismetMathLibrary.Normal` (- (`self.K2_GetActorLocation` _playershipref) _returnvalue_2)))) "Undefined" "OverrideRootScale" null null))
        (:`Is Not Valid`
          (`KismetSystemLibrary.Delay` 0.25)
          (goto _label))))
    (:`then_1`
      (`/Engine/EditorBlueprintResources/StandardMacros.IsValid` _playershipref_3 :!label _label_2
        (:`Is Valid`
          (`|SpawnActorFromClass` "/Game/Blueprints/BossFight/BP_BossMissile.BP_BossMissile_C" (`KismetMathLibrary.MakeTransform` _returnvalue_3 (`KismetMathLibrary.Conv_VectorToRotator` (`KismetMathLibrary.Normal` (- (`self.K2_GetActorLocation` _playershipref_3) _returnvalue_3)))) "Undefined" "OverrideRootScale" null null))
        (:`Is Not Valid`
          (`KismetSystemLibrary.Delay` 0.25)
          (goto _label_2))))
    (:`then_2`
      (`/Engine/EditorBlueprintResources/StandardMacros.IsValid` _playershipref_4 :!label _label_3
        (:`Is Valid`
          (`|SpawnActorFromClass` "/Game/Blueprints/BossFight/BP_BossMissile.BP_BossMissile_C" (`KismetMathLibrary.MakeTransform` _returnvalue_4 (`KismetMathLibrary.Conv_VectorToRotator` (`KismetMathLibrary.Normal` (- (`self.K2_GetActorLocation` _playershipref_4) _returnvalue_4)))) "Undefined" "OverrideRootScale" null null))
        (:`Is Not Valid`
          (`KismetSystemLibrary.Delay` 0.25)
          (goto _label_3))))
    (:`then_3`
      (`/Engine/EditorBlueprintResources/StandardMacros.IsValid` _playershipref_2 :!label _label_4
        (:`Is Valid`
          (`|SpawnActorFromClass` "/Game/Blueprints/BossFight/BP_BossMissile.BP_BossMissile_C" (`KismetMathLibrary.MakeTransform` _returnvalue (`KismetMathLibrary.Conv_VectorToRotator` (`KismetMathLibrary.Normal` (- (`self.K2_GetActorLocation` _playershipref_2) _returnvalue)))) "Undefined" "OverrideRootScale" null null))
        (:`Is Not Valid`
          (`KismetSystemLibrary.Delay` 0.25)
          (goto _label_4))))))

(fn `MainCannonChargeUp`
  (params (InDelta :type "Float (double-precision)"))
  (bind _output_get (set `self.MainCannonCooldownTimer` (+ InDelta (`self.MainCannonCooldownTimer`))))
  (if (> _output_get 22.5)
    (set `self.bCannonReady` true)
    (bind _output_get_2 (set `self.MainCannonChargeTimer` (+ InDelta (`self.MainCannonChargeTimer`))))
    (if (> _output_get_2 5.0)
      (`self.MainCannonFireEvent`)
      (set `self.MainCannonCooldownTimer` 0.0)
      (set `self.MainCannonChargeTimer` 0.0))))

(fn `MainCannonDealDamage`
  (for _array_element (`PrimitiveComponent.GetOverlappingActors` (`self.CannonBox`) "/Game/Blueprints/BP_PlayerPhoenix.BP_PlayerPhoenix_C")
    (bind _asjam_ship_base (cast `JamShipBase` _array_element))
    (`self.ShipApplyDamage` _asjam_ship_base (`self.CannonDamage`))
    (`KismetSystemLibrary.PrintString` (`KismetSystemLibrary.GetDisplayName` _array_element) true true (struct :`R` 1.0 :`G` 0.43924 :`A` 1.0) 20.0)))

(fn `MainCannonFire`
  (bind _physicsroot (`self.PhysicsRoot`))
  (`KismetSystemLibrary.PrintString` "Boss Cannon Firing!")
  (`NiagaraFunctionLibrary.SpawnSystemAttached` "/Game/VFX/NS_BossBeam.NS_BossBeam" _physicsroot "None" (`SceneComponent.GetSocketLocation` _physicsroot "MainCannon") (struct) "SnapToTarget" true)
  (`AudioComponent.Play` (`self.SFXBossBeam`) 0.0))

(fn `MissileVolley`
  (params (InDelta :type "Float (double-precision)"))
  (bind _output_get (set `self.MissileVolleyTimer` (+ InDelta (`self.MissileVolleyTimer`))))
  (if (> _output_get 10.0)
    (set `self.MissileVolleyTimer` 0.0)
    (`self.SpawnMissile`)))

(fn `SetBossStats`
  (bind _asbp_jam_game_instance (cast `/Game/Blueprints/BP_JamGameInstance` (`GameplayStatics.GetGameInstance`)))
  (set `self.bShieldEnabled` true)
  (switch `int` (`/Game/Blueprints/BP_JamGameInstance.Difficulty` _asbp_jam_game_instance)
    (:`0`
      (bind _output_get (set `self.MaxArmor` 20000.0))
      (set `self.CurrentArmor` _output_get)
      (bind _output_get_2 (set `self.MaxShield` 15000.0))
      (set `self.CurrentShield` _output_get_2)
      (set `self.MaxFighters` 2)
      (set `self.TurretsFirepower` 5.0)
      (set `self.TurretRange` 10000.0)
      (set `self.CannonDamage` 500.0)
      (set `self.MaxSpeed` 0.0)
      (set `self.TurnSpeed` 20.0))
    (:`1`
      (bind _output_get_3 (set `self.MaxArmor` 30000.0))
      (set `self.CurrentArmor` _output_get_3)
      (bind _output_get_4 (set `self.MaxShield` 20000.0))
      (set `self.CurrentShield` _output_get_4)
      (set `self.MaxFighters` 3)
      (set `self.TurretsFirepower` 10.0)
      (set `self.TurretRange` 10000.0)
      (set `self.CannonDamage` 1000.0)
      (set `self.MaxSpeed` 0.0)
      (set `self.TurnSpeed` 25.0))
    (:`2`
      (bind _output_get_5 (set `self.MaxArmor` 40000.0))
      (set `self.CurrentArmor` _output_get_5)
      (bind _output_get_6 (set `self.MaxShield` 30000.0))
      (set `self.CurrentShield` _output_get_6)
      (set `self.MaxFighters` 4)
      (set `self.TurretsFirepower` 15.0)
      (set `self.TurretRange` 10000.0)
      (set `self.CannonDamage` 2000.0)
      (set `self.MaxSpeed` 0.0)
      (set `self.TurnSpeed` 30.0))
    (:`3`
      (bind _output_get_7 (set `self.MaxArmor` 50000.0))
      (set `self.CurrentArmor` _output_get_7)
      (bind _output_get_8 (set `self.MaxShield` 40000.0))
      (set `self.CurrentShield` _output_get_8)
      (set `self.MaxFighters` 6)
      (set `self.TurretsFirepower` 20.0)
      (set `self.TurretRange` 10000.0)
      (set `self.CannonDamage` 9999.0)
      (set `self.MaxSpeed` 0.0)
      (set `self.TurnSpeed` 40.0))))

(fn `SetPlayerShipTargets`
  (bind _playershipref (`self.PlayerShipRef`))
  (`/Engine/EditorBlueprintResources/StandardMacros.IsValid` _playershipref
    (:`Is Valid`
      (set `self.TurretTargetShip` _playershipref))
    (:`Is Not Valid`
      (`KismetSystemLibrary.PrintString` "Failed to set turret target on boss ship." true false (struct :`R` 1.0 :`A` 1.0) 20.0))))

(fn `UserConstructionScript`)