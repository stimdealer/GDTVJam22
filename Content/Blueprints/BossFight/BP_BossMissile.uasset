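; BP_BossMissile is a boss-fight projectile that flies straight along its mesh's forward vector and damages the player's phoenix ship on contact.
; Tick moves it without sweep and destroys it after an eight-second lifetime.
; A capsule overlap with BP_PlayerPhoenix fires once, applying damage, spawning an explosion and sound, removing the mesh to halt movement, then destroying the actor after a short delay.
; BeginPlay scales the explosion volume from the game instance's effects setting.
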(event `self.ReceiveBeginPlay`
  (bind _asbp_jam_game_instance (cast `/Game/Blueprints/BP_JamGameInstance` (`GameplayStatics.GetGameInstance`)))
  (`AudioComponent.SetVolumeMultiplier` (`self.SFXExplode`) (`/Game/Blueprints/BP_JamGameInstance.EffectsVolPercent` _asbp_jam_game_instance)))

(event `self.ReceiveTick`
  (params (DeltaSeconds :type "Float (single-precision)"))
  (bind _missilemesh (`self.MissileMesh`))
  (set `self.LifeTimer` (+ DeltaSeconds (`self.LifeTimer`)))
  (`/Engine/EditorBlueprintResources/StandardMacros.IsValid` _missilemesh
    (:`Is Valid`
      (`self.K2_AddActorWorldOffset` (* (`SceneComponent.GetForwardVector` _missilemesh) 2000.0 DeltaSeconds)))
    (:`Is Not Valid`
      _))
  (if (> (`self.LifeTimer`) 8.0)
    (`self.K2_DestroyActor`)))

(event `self.TriggerCapsule.OnComponentBeginOverlap`
  (params (OverlappedComponent :type "PrimitiveComponent Object Reference") (OtherActor :type "Actor Object Reference") (OtherComp :type "PrimitiveComponent Object Reference") (OtherBodyIndex :type Integer) (bFromSweep :type Boolean) (SweepResult :type "HitResult Structure (by ref)"))
  (bind _asbp_player_phoenix (cast `/Game/Blueprints/BP_PlayerPhoenix` OtherActor))
  (`/Engine/EditorBlueprintResources/StandardMacros.DoOnce` false
    (:`Completed`
      (`JamShipBase.ShipApplyDamage` _asbp_player_phoenix 150.0)
      (`NiagaraFunctionLibrary.SpawnSystemAtLocation` "/Game/VFX/NS_GeneralExplosion.NS_GeneralExplosion" (`self.K2_GetActorLocation` self))
      (`AudioComponent.Play` (`self.SFXExplode`) 0.0)
      (`ActorComponent.K2_DestroyComponent` (`self.MissileMesh`))
      (`KismetSystemLibrary.Delay` 1.5)
      (`self.K2_DestroyActor`))))

(fn `UserConstructionScript`)