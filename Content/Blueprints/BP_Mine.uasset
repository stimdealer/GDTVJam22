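; BP_Mine is a mine that homes in on the player ship and destroys itself when a ship gets close.
; Entering or leaving the ProximitySphere toggles pursuit and the glow on a dynamic material instance.
; While pursuing, Tick pushes MineMesh toward the player with a mass-independent force.
; Any JamShipBase entering the TriggerSphere destroys the mine; explosion VFX is only a comment, and the overlapping-ship loop applies no effect.
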(event `self.ReceiveTick`
  (params (DeltaSeconds :type "Float (single-precision)"))
  (if (`self.bPursuePlayer`)
    (`PrimitiveComponent.AddForce` (`self.MineMesh`) (* (`KismetMathLibrary.Normal` (- (`self.K2_GetActorLocation` (`self.PlayerShip`)) (`self.K2_GetActorLocation`))) 200.0) "None" true)))

(event `self.ReceiveBeginPlay`
  (bind _minemesh (`self.MineMesh`))
  (bind _returnvalue (`KismetMaterialLibrary.CreateDynamicMaterialInstance` (`StaticMesh.GetMaterial` (`StaticMeshComponent.StaticMesh` _minemesh) 0)))
  (bind _output_get (set `self.MineDynamicMaterial` _returnvalue))
  (`MaterialInstanceDynamic.SetScalarParameterValue` _output_get "Glow" 0.0)
  (`PrimitiveComponent.SetMaterial` _minemesh 0 _output_get))

(event `self.ProximitySphere.OnComponentBeginOverlap`
  (params (OverlappedComponent :type "PrimitiveComponent Object Reference") (OtherActor :type "Actor Object Reference") (OtherComp :type "PrimitiveComponent Object Reference") (OtherBodyIndex :type Integer) (bFromSweep :type Boolean) (SweepResult :type "HitResult Structure (by ref)"))
  (bind _asbp_player_ship (cast `/Game/Blueprints/BP_PlayerShip` OtherActor))
  (set `self.PlayerShip` _asbp_player_ship)
  (`MaterialInstanceDynamic.SetScalarParameterValue` (`self.MineDynamicMaterial`) "Glow" 50.0)
  (set `self.bPursuePlayer` true))

(event `self.ProximitySphere.OnComponentEndOverlap`
  (params (OverlappedComponent :type "PrimitiveComponent Object Reference") (OtherActor :type "Actor Object Reference") (OtherComp :type "PrimitiveComponent Object Reference") (OtherBodyIndex :type Integer))
  (cast `/Game/Blueprints/BP_PlayerShip` OtherActor)
  (`MaterialInstanceDynamic.SetScalarParameterValue` (`self.MineDynamicMaterial`) "Glow" 0.0)
  (set `self.bPursuePlayer` false))

(event `self.TriggerSphere.OnComponentBeginOverlap`
  (params (OverlappedComponent :type "PrimitiveComponent Object Reference") (OtherActor :type "Actor Object Reference") (OtherComp :type "PrimitiveComponent Object Reference") (OtherBodyIndex :type Integer) (bFromSweep :type Boolean) (SweepResult :type "HitResult Structure (by ref)"))
  (cast `JamShipBase` OtherActor)
  (for _array_element (`PrimitiveComponent.GetOverlappingActors` (`self.TriggerSphere`) null)
    (cast `JamShipBase` _array_element))
  ;[1 1 1] Spawn Explosion VFX
  (`self.K2_DestroyActor` self))

(fn `UserConstructionScript`)