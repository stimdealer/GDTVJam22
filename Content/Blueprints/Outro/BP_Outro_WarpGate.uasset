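; BP_Outro_WarpGate is the outro's warp gate, which lights up and shows a spinning funnel.
; BeginPlay creates a dynamic material on the gate mesh, then immediately calls BossDeath, which raises Glow, reveals WarpFunnel and sets GateActive.
; While GateActive is true, Tick rolls the funnel at a constant, frame-rate-independent speed.
; A node that would zero Glow is left unconnected, so the gate starts active.
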(event `self.ReceiveBeginPlay`
  (bind _warpgatemesh (`self.WarpGateMesh`))
  (bind _returnvalue (`PrimitiveComponent.CreateDynamicMaterialInstance` _warpgatemesh 0 (`PrimitiveComponent.GetMaterial` _warpgatemesh 0) "None"))
  (set `self.DynamicMaterial` _returnvalue)
  (`self.BossDeath`))

(event `self.ReceiveTick`
  (params (DeltaSeconds :type "Float (single-precision)"))
  (if (`self.bGateActive`)
    (`SceneComponent.K2_AddLocalRotation` (`self.WarpFunnel`) (`KismetMathLibrary.MakeRotator` (* DeltaSeconds 30.0)) false false)))

(fn `BossDeath`
  (`MaterialInstanceDynamic.SetScalarParameterValue` (`self.DynamicMaterial`) "Glow" 20.0)
  (set `self.bGateActive` true)
  (`SceneComponent.SetVisibility` (`self.WarpFunnel`) true false))

(fn `UserConstructionScript`)