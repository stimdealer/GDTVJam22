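; BP_Intro_HeroShip is the hero ship actor for the game's intro, handling skip input, music and the handoff to the StarMap level.
; BeginPlay shows the WBP_IntroSkip widget, and Space or Escape opens StarMap immediately.
; EventStartMusic activates intro music at the volume stored in BP_JamGameInstance, while LoadLevel opens StarMap; neither is called within this Blueprint.
; Looping ship movement logic remains in the graph but is disconnected.
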(event `self.ReceiveBeginPlay`
  (bind _returnvalue (`|CreateWidget` "/Game/UI/WBP_IntroSkip.WBP_IntroSkip_C" (`GameplayStatics.GetPlayerController` 0)))
  (`UserWidget.AddToViewport` _returnvalue 0))

(event `self.ReceiveTick`
  (params (DeltaSeconds :type "Float (single-precision)")))

(event `EventStartMusic`
  (bind _asbp_jam_game_instance (cast `/Game/Blueprints/BP_JamGameInstance` (`GameplayStatics.GetGameInstance`)))
  (`AudioComponent.SetVolumeMultiplier` (`self.IntroMusic`) (* (`/Game/Blueprints/BP_JamGameInstance.MusicVolPercent` _asbp_jam_game_instance) (`/Game/Blueprints/BP_JamGameInstance.MusicVolumeMult` _asbp_jam_game_instance)))
  (`ActorComponent.Activate` (`self.IntroMusic`) false))

(event `LoadLevel`
  (`GameplayStatics.OpenLevel` "StarMap"))

(event `Key|SpaceBar`
  (params (Key :type "Key Structure"))
  (:`Pressed`
    (`GameplayStatics.OpenLevel` "StarMap" :!label _label)))

(event `Key|Escape`
  (params (Key :type "Key Structure"))
  (:`Pressed`
    (goto _label)))

(fn `UserConstructionScript`)