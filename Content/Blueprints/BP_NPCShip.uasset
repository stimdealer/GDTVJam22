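; BP_NPCShip is an NPC ship with a turret, target-marker arrows and shield/armor status bars.
; BeginPlay registers Turret01 in the Turrets array, and ToggleArrows shows or hides the arrows and bars together.
; While the arrows are visible, Tick spins them and pulses their scale by sampling a float curve on a looping one-second timer.
; UpdateStats passes shield and armor percentages to the WBP_EnemyBars widget.
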(event `self.ReceiveBeginPlay`
  (`KismetArrayLibrary.Array_Add` (`self.Turrets`) (`self.Turret_01`)))

(event `self.ReceiveTick`
  (params (DeltaSeconds :type "Float (single-precision)"))
  (`self.AnimateTargetArrows` DeltaSeconds))

(event `self.ToggleArrows`
  (params (IsVisible :type Boolean))
  (`SceneComponent.SetVisibility` (`self.TargetArrowsMesh`) IsVisible true)
  (`SceneComponent.SetVisibility` (`self.StatusBars`) IsVisible true))

(event `self.UpdateStats`
  (params (InShieldPercent :type "Float (single-precision)") (InArmorPercent :type "Float (single-precision)"))
  (bind _aswbp_enemy_bars (cast `/Game/UI/WBP_EnemyBars` (`WidgetComponent.GetWidget` (`self.StatusBars`))))
  (`/Game/UI/WBP_EnemyBars.SetStats` _aswbp_enemy_bars InShieldPercent InArmorPercent))

(fn `AnimateTargetArrows`
  (params (InDelta :type "Float (double-precision)"))
  (bind _targetarrowsmesh (`self.TargetArrowsMesh`))
  (if (`SceneComponent.bVisible` _targetarrowsmesh)
    (`SceneComponent.K2_AddLocalRotation` _targetarrowsmesh (`KismetMathLibrary.MakeRotator` 0.0 0.0 (* InDelta 50.0)) false false)
    (bind _output_get (set `self.PulseTimer` (+ InDelta (`self.PulseTimer`))))
    (bind _returnvalue (`CurveFloat.GetFloatValue` (`self.Curve`) _output_get))
    (`SceneComponent.SetRelativeScale3D` _targetarrowsmesh (`KismetMathLibrary.MakeVector` _returnvalue _returnvalue _returnvalue))
    (if (> _output_get 1.0)
      (set `self.PulseTimer` 0.0))))

(fn `UserConstructionScript`)