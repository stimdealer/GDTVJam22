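; Player ship Blueprint with a Phoenix system that damages nearby ships in a nova, then reconstitutes the ship.
; Cursor object traces feed navigation, target selection and timed-reload tracking missiles.
; Events launch fighters, handle permanent death with a menu, and relay stats, messages and quest markers to the UI.
; Audio takes volumes from the game instance, with cross-resetting DoOnce pairs switching looping thruster and weapon sounds only on state changes.
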(event `self.ReceiveBeginPlay`
  (bind _turrets (`self.Turrets`))
  (`KismetArrayLibrary.Array_Add` _turrets (`self.Turret_1`))
  (`KismetArrayLibrary.Array_Add` _turrets (`self.Turret_2`))
  (`self.SpawnWeaponsVFX`)
  (`self.BP_SetupAudio`))

(event `self.ReceiveTick`
  (params (DeltaSeconds :type "Float (single-precision)"))
  (`SceneComponent.K2_AddLocalRotation` (`self.TargetRing`) (`KismetMathLibrary.MakeRotator` 0.0 0.0 (* DeltaSeconds 20.0)) false false)
  (`self.BP_ClickNavTrace`)
  (`self.BP_MissileReload` DeltaSeconds))

(event `InputAction|PrimaryAction`
  (params (Key :type "Key Structure"))
  (:`Pressed`
    (bind _asjam_ship_base (`self.BP_GetTargetUnderMouse`))
    (`self.ManualSelectTarget` _asjam_ship_base)))

(event `InputAction|FireMissile`
  (params (Key :type "Key Structure"))
  (:`Pressed`
    (bind _asjam_ship_base (`self.BP_GetTargetUnderMouse`))
    (`self.BP_FireMissile` _asjam_ship_base)))

(event `self.PhoenixExplosion`
  (bind _physicsroot (`self.PhysicsRoot`))
  (`NiagaraFunctionLibrary.SpawnSystemAttached` "/Game/VFX/NS_PhoenixNova.NS_PhoenixNova" (`self.PhysicsRoot`) "None" (`self.K2_GetActorLocation` self) (struct) "SnapToTarget" true)
  (`PlayerController.ClientStartCameraShake` :`self` (`GameplayStatics.GetPlayerController` 0) :`Shake` "/Game/Blueprints/BP_CameraShakeBig.BP_CameraShakeBig_C")
  (`AudioComponent.Play` (`self.SFXPhoenixExplode`) 0.0)
  (set `self.bPhoenixInProgress` true)
  (`PrimitiveComponent.SetSimulatePhysics` _physicsroot false)
  (`PrimitiveComponent.SetPhysicsLinearVelocity` _physicsroot (0.0 0.0 0.0) false "None")
  (for _array_element (`PrimitiveComponent.GetOverlappingActors` (`self.PhoenixExplosionSphere`) null)
    (bind _asjam_ship_base (cast `JamShipBase` _array_element))
    (`self.ShipApplyDamage` _asjam_ship_base 500.0))
  (`KismetSystemLibrary.Delay` 3.0)
  (`AudioComponent.Play` (`self.SFXPhoenixDischarging`) 0.0)
  (`self.BP_SendMessageToUI` "FIrst Officer: Phoenix system activated. Ship has been reconstituted with minimal abilities." true)
  (`PrimitiveComponent.SetSimulatePhysics` (`self.PhysicsRoot`) true)
  (set `self.bPhoenixInProgress` false))

(event `self.ShipPermanentDeath`
  (bind _returnvalue (`GameplayStatics.GetPlayerController` 0))
  (`NiagaraFunctionLibrary.SpawnSystemAttached` "/Game/VFX/NS_PlayerShipExplosion.NS_PlayerShipExplosion" (`self.PhysicsRoot`) "None" (0.0 0.0 0.0) (struct) "SnapToTarget" true)
  (`PlayerController.ClientStartCameraShake` :`self` (`GameplayStatics.GetPlayerController` 0) :`Shake` "/Game/Blueprints/BP_CameraShakeBig.BP_CameraShakeBig_C")
  (`AudioComponent.Play` (`self.SFXShipExplode`) 0.0)
  (`AudioComponent.FadeOut` (`self.Music`) 0.5 0.0 "Linear")
  (`KismetSystemLibrary.Delay` 3.0)
  (bind _returnvalue_2 (`|CreateWidget` "/Game/UI/WBP_DeathMenu.WBP_DeathMenu_C" _returnvalue))
  (`UserWidget.AddToViewport` _returnvalue_2 0)
  (`WidgetBlueprintLibrary.SetInputMode_UIOnlyEx` _returnvalue null)
  (`self.K2_DestroyActor`))

(event `self.LaunchFighter`
  (params (InTarget :type "NPCShip Object Reference"))
  (bind _returnvalue (`|SpawnActorFromClass` "/Game/Blueprints/BP_PlayerFighter.BP_PlayerFighter_C" (`KismetMathLibrary.MakeTransform` (`SceneComponent.GetSocketLocation` (`self.PhysicsRoot`) "Fighter_Bay")) "AdjustIfPossibleButAlwaysSpawn" "OverrideRootScale" null null))
  (`FighterShip.AssignTarget` _returnvalue InTarget self)
  (`KismetArrayLibrary.Array_Add` (`self.DeployedFighters`) _returnvalue))

(event `self.SendArmorFuelToUI`
  (params (InShieldPercent :type "Float (single-precision)") (InArmorPercent :type "Float (single-precision)") (InFuelPercent :type "Float (single-precision)") (InOrePercent :type "Float (single-precision)") (InPhoenixPercent :type "Float (single-precision)"))
  (bind _playerhud (`self.PlayerHUD`))
  (`/Engine/EditorBlueprintResources/StandardMacros.IsValid` _playerhud
    (:`Is Valid`
      (`/Game/UI/WBP_MainGameHUD.UpdateBarStats` _playerhud InShieldPercent InArmorPercent InFuelPercent InOrePercent InPhoenixPercent))))

(event `self.SendIconsToUI`
  (params (InBroadsides :type Boolean) (InMissiles :type Boolean) (InFighters :type Boolean) (InMissileReady :type Boolean))
  (bind _playerhud (`self.PlayerHUD`))
  (`/Engine/EditorBlueprintResources/StandardMacros.IsValid` _playerhud
    (:`Is Valid`
      (`/Game/UI/WBP_MainGameHUD.UpdateIcons` _playerhud InBroadsides (and InMissiles InMissileReady) InFighters))))

(event `self.SendMessageToUI`
  (params (InMessage :type "Text (by ref)") (bCommMessage :type Boolean))
  (`self.BP_SendMessageToUI` InMessage bCommMessage))

(event `self.SFXThruster`
  (params (IsBoosting :type Boolean))
  (bind _sfxboosters (`self.SFXBoosters`))
  (bind _sfxthrusters (`self.SFXThrusters`))
  (if IsBoosting
    (`/Engine/EditorBlueprintResources/StandardMacros.DoOnce` false :!label _label
      (:`Completed`
        (`AudioComponent.Play` _sfxboosters 0.0)
        (`AudioComponent.Stop` _sfxthrusters)
        (goto _label_2 :!via `Reset`)))
    (else
      (`/Engine/EditorBlueprintResources/StandardMacros.DoOnce` false :!label _label_2
        (:`Completed`
          (`AudioComponent.Play` _sfxthrusters 0.0)
          (`AudioComponent.Stop` _sfxboosters)
          (goto _label :!via `Reset`))))))

(event `self.SFXImpactDamage`
  (params (IsShieldImpact :type Boolean))
  (if IsShieldImpact
    (`AudioComponent.Play` (`self.SFXShieldImpact`) 0.0)
    (else
      (`AudioComponent.Play` (`self.SFXImpact`) 0.0))))

(event `self.SFXTurretsFiring`
  (params (IsActive :type Boolean))
  (bind _sfxturrets (`self.SFXTurrets`))
  (if IsActive
    (`/Engine/EditorBlueprintResources/StandardMacros.DoOnce` false :!label _label_3
      (:`Completed`
        (`AudioComponent.Play` _sfxturrets 0.0)
        (goto _label_4 :!via `Reset`)))
    (else
      (`/Engine/EditorBlueprintResources/StandardMacros.DoOnce` false :!label _label_4
        (:`Completed`
          (`AudioComponent.Stop` _sfxturrets)
          (goto _label_3 :!via `Reset`))))))

(event `self.SFXBroadsidesFiring`
  (params (IsActive :type Boolean))
  (bind _sfxbroadsides (`self.SFXBroadsides`))
  (if IsActive
    (`/Engine/EditorBlueprintResources/StandardMacros.DoOnce` false :!label _label_5
      (:`Completed`
        (`AudioComponent.Play` _sfxbroadsides 0.0)
        (goto _label_6 :!via `Reset`)))
    (else
      (`/Engine/EditorBlueprintResources/StandardMacros.DoOnce` false :!label _label_6
        (:`Completed`
          (`AudioComponent.Stop` _sfxbroadsides)
          (goto _label_5 :!via `Reset`))))))

(fn `BP_ClickNavTrace`
  (bind (_bblockinghit _binitialoverlap _time _distance _location) (`GameplayStatics.BreakHitResult` (`PlayerController.GetHitResultUnderCursorForObjects` (`GameplayStatics.GetPlayerController` 0) (`|MakeArray` "ObjectTypeQuery8" :!type "EObjectTypeQuery Enum") false)))
  (if _bblockinghit
    (bind _output_get (set `self.Destination` _location))))

(fn `BP_FireMissile`
  (params (InTarget :type "JamShipBase Object Reference"))
  (if (and (`self.bLauncher`) (`self.bMissileReady`))
    (`/Engine/EditorBlueprintResources/StandardMacros.IsValid` InTarget
      (:`Is Valid`
        (bind _returnvalue (`|SpawnActorFromClass` "/Script/GameJam.TrackingMissile" (`KismetMathLibrary.MakeTransform` (`SceneComponent.GetSocketLocation` (`self.PhysicsRoot`) "Launcher")) "AlwaysSpawn" "OverrideRootScale" null null))
        (set `TrackingMissile.Target` InTarget _returnvalue)
        (set `self.bMissileReady` false)
        (`AudioComponent.Play` (`self.SFXMissileLaunch`) 0.0))
      (:`Is Not Valid`
        (`self.BP_SendMessageToUI` "Weapons Officer: Please mouse over a target ship to launch a missile at them." true)))
    (else
      (`self.BP_SendMessageToUI` "Weapons Officer: Our next missile is not ready yet, captain." true))))

(fn `BP_GetTargetUnderMouse`
  (returns (`AsJam Ship Base` :type "JamShipBase Object Reference"))
  (bind (_bblockinghit _binitialoverlap _time _distance _location _impactpoint _normal _impactnormal _physmat _hitactor) (`GameplayStatics.BreakHitResult` (`PlayerController.GetHitResultUnderCursorForObjects` (`GameplayStatics.GetPlayerController` 0) (`|MakeArray` "ObjectTypeQuery8" :!type "EObjectTypeQuery Enum") true)))
  (if (!= self _hitactor)
    (bind _asjam_ship_base (cast `JamShipBase` _hitactor)
      (:`then`
        (return _asjam_ship_base))
      (:`CastFailed`
        _)))
  (return null))

(fn `BP_MissileReload`
  (params (A :type "Float (double-precision)"))
  (if (not (`self.bMissileReady`))
    (bind _output_get (set `self.MissileReloadTimer` (+ A (`self.MissileReloadTimer`))))
    (if (> _output_get 5.0)
      (set `self.bMissileReady` true)
      (set `self.MissileReloadTimer` 0.0))))

(fn `BP_PhoenixExplosion`)

(fn `BP_SendMessageToUI`
  (params (NewItem :type "Text (by ref)") (CommMessage :type Boolean))
  (bind _playerhud (`self.PlayerHUD`))
  (`/Engine/EditorBlueprintResources/StandardMacros.IsValid` _playerhud
    (:`Is Valid`
      (if CommMessage
        (`/Game/UI/WBP_MainGameHUD.AddCommMessage` _playerhud NewItem)
        (else
          (`KismetArrayLibrary.Array_Add` (`/Game/UI/WBP_MainGameHUD.MessageBuffer` _playerhud) NewItem))))))

(fn `BP_SetQuestMarkerPosition`
  (params (InPosition :type "Vector2D Structure") (InWidget :type "/Game/UI/Components/WBP_QuestMarker Object Reference"))
  (locals (QuestIconRadius :type "Float (double-precision)" :default 60.0) (NewX :type "Float (double-precision)") (NewY :type "Float (double-precision)"))
  (bind (_returnvalue_x _returnvalue_y) (`KismetMathLibrary.BreakVector2D` (`WidgetLayoutLibrary.GetViewportSize`)))
  (bind _questiconradius (`local.QuestIconRadius`))
  (`|ExecutionSequence`
    (:`then_0`
      (if (> InPosition_X _returnvalue_x)
        (set `local.NewX` (- _returnvalue_x _questiconradius))
        (elif (< (- InPosition_X _questiconradius) 0.0)
          (set `local.NewX` 0.0)
          (else
            (set `local.NewX` (- InPosition_X _questiconradius))))))
    (:`then_1`
      (if (> InPosition_Y _returnvalue_y)
        (set `local.NewY` (- _returnvalue_y _questiconradius))
        (elif (< (- InPosition_Y _questiconradius) 0.0)
          (set `local.NewY` 0.0)
          (else
            (set `local.NewY` (- InPosition_Y _questiconradius))))))
    (:`then_2`
      (`UserWidget.SetPositionInViewport` InWidget (`KismetMathLibrary.MakeVector2D` (`local.NewX`) (`local.NewY`)) true))))

(fn `BP_SetupAudio`
  (bind _music (`self.Music`))
  (bind _asbp_jam_game_instance (cast `/Game/Blueprints/BP_JamGameInstance` (`GameplayStatics.GetGameInstance`)))
  (`|ExecutionSequence`
    (:`then_0`
      (`AudioComponent.SetSound` _music "/Game/SFX/Cue_InGameMusic.Cue_InGameMusic")
      (`AudioComponent.SetVolumeMultiplier` _music (* (`/Game/Blueprints/BP_JamGameInstance.MusicVolPercent` _asbp_jam_game_instance) (`/Game/Blueprints/BP_JamGameInstance.MusicVolumeMult` _asbp_jam_game_instance)))
      (`AudioComponent.Play` _music 0.0))
    (:`then_1`
      (bind _effectsvolpercent (`/Game/Blueprints/BP_JamGameInstance.EffectsVolPercent` _asbp_jam_game_instance))
      (`AudioComponent.SetVolumeMultiplier` (`self.SFXPhoenixExplode`) _effectsvolpercent)
      (`AudioComponent.SetVolumeMultiplier` (`self.SFXShipExplode`) _effectsvolpercent)
      (`AudioComponent.SetVolumeMultiplier` (`self.SFXBroadsides`) _effectsvolpercent)
      (`AudioComponent.SetVolumeMultiplier` (`self.SFXTurrets`) _effectsvolpercent))
    (:`then_2`
      (`AudioComponent.SetVolumeMultiplier` (`self.SFXMissileLaunch`) _effectsvolpercent)
      (`AudioComponent.SetVolumeMultiplier` (`self.SFXImpact`) _effectsvolpercent)
      (`AudioComponent.SetVolumeMultiplier` (`self.SFXShieldImpact`) _effectsvolpercent)
      (`AudioComponent.SetVolumeMultiplier` (`self.SFXShipAmbience`) _effectsvolpercent))
    (:`then_3`
      (`AudioComponent.SetVolumeMultiplier` (`self.SFXPhoenixDischarging`) _effectsvolpercent)
      (`AudioComponent.SetVolumeMultiplier` (`self.SFXPhoenixRecharged`) _effectsvolpercent))))

(fn `BP_UpdateMarkerWidget`
  (params (InQuestName :type "String (by ref)") (InPosition :type "Vector2D Structure") (InIconType :type Integer) (Enlarged :type Boolean))
  (locals (FoundWidget :type "/Game/UI/Components/WBP_QuestMarker Object Reference"))
  (bind _foundwidget (`local.FoundWidget`))
  (bind (_value _returnvalue) (`BlueprintMapLibrary.Map_Find` (`self.QuestMarkers`) InQuestName))
  (`|ExecutionSequence`
    (:`then_0`
      (if _returnvalue
        (set `local.FoundWidget` _value)
        (else
          (bind _returnvalue_2 (`|CreateWidget` "/Game/UI/Components/WBP_QuestMarker.WBP_QuestMarker_C" (`GameplayStatics.GetPlayerController` 0)))
          (`/Game/UI/Components/WBP_QuestMarker.SetIconType` _returnvalue_2 InIconType)
          (`UserWidget.AddToViewport` _returnvalue_2 0)
          (`BlueprintMapLibrary.Map_Add` (`self.QuestMarkers`) InQuestName _returnvalue_2)
          (set `local.FoundWidget` _returnvalue_2))))
    (:`then_1`
      (`/Game/UI/Components/WBP_QuestMarker.EnlargeIcon` _foundwidget Enlarged)
      (`UserWidget.SetPositionInViewport` _foundwidget InPosition true))))

(fn `UserConstructionScript`)