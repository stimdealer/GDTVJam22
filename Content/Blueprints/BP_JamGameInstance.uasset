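; BP_JamGameInstance is the game instance that runs the level's quest flow: repair every relay station, then reach the warp gate.
; It creates a numbered repair quest on the player ship for each relay station actor, maps each relay to its quest name, and records the total.
; Each repaired relay completes its quest; once all are done, it activates the warp gates, posts comm messages and adds the gate quest.
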(fn `CheckQuestRelayRepaired`
  (params (InRelayRef :type "/Game/Blueprints/Environment/BP_RelayStation Object Reference"))
  (`/Engine/EditorBlueprintResources/StandardMacros.IncrementInt` (`self.RelaysRepaired`)
    (:`  `
      (`PlayerShip.CompleteQuest` (`self.PlayerShipRef`) (`BlueprintMapLibrary.Map_Find` (`self.ActiveQuests`) InRelayRef))
      (if (>= (`self.RelaysRepaired`) (`self.TotalRelays`))
        (`self.GenerateWarpGateQuest`)))))

(fn `GenerateRelayQuests`
  (`/Engine/EditorBlueprintResources/StandardMacros.IsValid` (`self.PlayerShipRef`)
    (:`Is Valid`
      (bind _outactors (`GameplayStatics.GetAllActorsOfClass` "/Game/Blueprints/Environment/BP_RelayStation.BP_RelayStation_C"))
      (for (_array_element _array_index) _outactors
        (bind _returnvalue (`KismetStringLibrary.Concat_StrStr` "Repair Relay Station " (`KismetStringLibrary.Conv_IntToString` (+ _array_index 1))))
        (`BlueprintMapLibrary.Map_Add` (`self.ActiveQuests`) _array_element _returnvalue)
        (`PlayerShip.AddQuest` (`self.PlayerShipRef`) _returnvalue (`Actor.K2_GetActorLocation` _array_element)))
      (set `self.TotalRelays` (`KismetArrayLibrary.Array_Length` _outactors)))))

(fn `GenerateWarpGateQuest`
  (bind _playershipref (`self.PlayerShipRef`))
  (bind _outactors (`GameplayStatics.GetAllActorsOfClass` "/Game/Blueprints/Environment/BP_WarpGate.BP_WarpGate_C"))
  (for _array_element _outactors
    (`/Engine/EditorBlueprintResources/StandardMacros.IsValid` _array_element
      (:`Is Valid`
        (`/Game/Blueprints/BP_PlayerPhoenix.BP_SendMessageToUI` _playershipref "Chief Engineer: The last relay has been repaird. The warp gate is online!" true)
        (`/Game/Blueprints/BP_PlayerPhoenix.BP_SendMessageToUI` _playershipref "All relays are repaird. The warp gate is online." true)
        (`/Game/Blueprints/Environment/BP_WarpGate.ActivateWarpGate` _array_element)
        (`PlayerShip.AddQuest` (`self.PlayerShipRef`) "Reach the Warp Gate" (`Actor.K2_GetActorLocation` _array_element))))))