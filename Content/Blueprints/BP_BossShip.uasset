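; Boss ship enemy with armor, shields, fighters, turrets and a missile attack.
; SetBossStats scales armor, shield and fighter cap from the game instance's Difficulty and fixes movement at zero speed with a set turn rate.
; UpdateStats pushes the armor percentage to the WBP_EnemyBars status widget.
; MissileVolley spawns a BP_BossMissile, and ToggleTeleTurrets shows or hides the center, port and starboard Tell turret components.
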(event `self.ReceiveBeginPlay`
  (`KismetArrayLibrary.Array_Add` (`self.Turrets`)))

(event `self.ReceiveTick`
  (params (DeltaSeconds :type "Float (single-precision)")))

(event `self.UpdateStats`
  (params (InArmorPercent :type "Float (single-precision)"))
  (bind _aswbp_enemy_bars (cast `/Game/UI/WBP_EnemyBars` (`WidgetComponent.GetWidget` (`self.StatusBars`))))
  (`/Game/UI/WBP_EnemyBars.SetStats` _aswbp_enemy_bars InArmorPercent))

(fn `MissileVolley`
  (`|SpawnActorFromClass` "/Game/Blueprints/BossFight/BP_BossMissile.BP_BossMissile_C" (`KismetMathLibrary.MakeTransform` (0.0 0.0 0.0)) "Undefined" "OverrideRootScale" null null))

(fn `SetBossStats`
  (bind _asbp_jam_game_instance (cast `/Game/Blueprints/BP_JamGameInstance` (`GameplayStatics.GetGameInstance`)))
  (bind _difficulty (`/Game/Blueprints/BP_JamGameInstance.Difficulty` _asbp_jam_game_instance))
  (bind _returnvalue (`KismetMathLibrary.Conv_IntToDouble` (* _difficulty 4000)))
  (set `self.MaxArmor` _returnvalue)
  (set `self.CurrentArmor` _returnvalue)
  (bind _returnvalue_2 (`KismetMathLibrary.Conv_IntToDouble` (* _difficulty 2000)))
  (set `self.MaxShield` _returnvalue_2)
  (set `self.CurrentShield` _returnvalue_2)
  (set `self.MaxFighters` (* _difficulty 3))
  (set `self.MaxSpeed` 0.0)
  (set `self.TurnSpeed` 20.0))

(fn `ToggleTeleTurrets`
  (params (InActive :type Boolean))
  (`SceneComponent.SetVisibility` (`self.TellCenterTurrets`) InActive false)
  (`SceneComponent.SetVisibility` (`self.TellPortTurrets`) InActive false)
  (`SceneComponent.SetVisibility` (`self.TellStbdTurrets`) InActive false))

(fn `UserConstructionScript`)