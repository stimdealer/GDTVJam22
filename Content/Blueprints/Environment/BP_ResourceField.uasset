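; Resource field actor that scatters loot asteroid ore around its location when play begins.
; The construction script adds mesh instances as an editor preview, offsetting them only in X and Y.
; On BeginPlay it destroys the preview and spawns Amount ore actors at random 3D offsets within a min/max spacing.
; Both passes draw directions and distances from the Seed random stream.
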(event `self.ReceiveBeginPlay`
  (bind _seed (`self.Seed`))
  (`ActorComponent.K2_DestroyComponent` (`self.MeshPreviews`))
  (for _ (range 1 (+ (`self.Amount`) 1))
    (`|SpawnActorFromClass` "/Game/Blueprints/Environment/Components/BP_LootAsteroidOre.BP_LootAsteroidOre_C" (`KismetMathLibrary.MakeTransform` (+ (* (`KismetMathLibrary.RandomUnitVectorFromStream` _seed) (`KismetMathLibrary.RandomFloatInRangeFromStream` (`self.MinSpacing`) (`self.MaxSpacing`) _seed)) (`self.K2_GetActorLocation` self))) "AdjustIfPossibleButAlwaysSpawn" "OverrideRootScale" null null)))

(fn `UserConstructionScript`
  (bind _seed (`self.Seed`))
  (bind (_returnvalue_x _returnvalue_y) (`KismetMathLibrary.BreakVector` (* (`KismetMathLibrary.RandomUnitVectorFromStream` _seed) (`KismetMathLibrary.RandomFloatInRangeFromStream` (`self.MinSpacing`) (`self.MaxSpacing`) _seed))))
  (for _ (range 1 (+ (`self.Amount`) 1))
    (`InstancedStaticMeshComponent.AddInstance` (`self.MeshPreviews`) (`KismetMathLibrary.MakeTransform` (`KismetMathLibrary.MakeVector` _returnvalue_x _returnvalue_y)) false)))