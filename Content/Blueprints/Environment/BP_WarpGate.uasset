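; BP_WarpGate is the level's escape gate, which stays offline until a dreadnought boss is defeated.
; ActivateWarpGate enables the rear blocker and arms the encounter, so player entry into the area box spawns BP_BossShip once with a back-reference to the gate.
; BossDeath lights the dynamic material, reveals the spinning funnel and fades in portal audio.
; Entering the active gate shows the victory menu, then destroys the player ship after a delay.
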(event `self.ReceiveBeginPlay`
  (bind _warpgatemesh (`self.WarpGateMesh`))
  (bind _returnvalue (`PrimitiveComponent.CreateDynamicMaterialInstance` _warpgatemesh 0 (`PrimitiveComponent.GetMaterial` _warpgatemesh 0) "None"))
  (set `self.DynamicMaterial` _returnvalue)
  (`MaterialInstanceDynamic.SetScalarParameterValue` _returnvalue "Glow" 0.0)
  (bind _asbp_jam_game_instance (cast `/Game/Blueprints/BP_JamGameInstance` (`GameplayStatics.GetGameInstance`)))
  (`AudioComponent.SetVolumeMultiplier` (`self.SFXPortal`) (`/Game/Blueprints/BP_JamGameInstance.EffectsVolPercent` _asbp_jam_game_instance)))

(event `self.ReceiveTick`
  (params (DeltaSeconds :type "Float (single-precision)"))
  (if (`self.bGateActive`)
    (`SceneComponent.K2_AddLocalRotation` (`self.WarpFunnel`) (`KismetMathLibrary.MakeRotator` (* DeltaSeconds 30.0)) false false)))

(event `self.WarpGateEnter.OnComponentBeginOverlap`
  (params (OverlappedComponent :type "PrimitiveComponent Object Reference") (OtherActor :type "Actor Object Reference") (OtherComp :type "PrimitiveComponent Object Reference") (OtherBodyIndex :type Integer) (bFromSweep :type Boolean) (SweepResult :type "HitResult Structure (by ref)"))
  (bind _returnvalue (`GameplayStatics.GetPlayerController` 0))
  (bind _asbp_player_phoenix (cast `/Game/Blueprints/BP_PlayerPhoenix` OtherActor))
  (if (`self.bGateActive`)
    (bind _returnvalue_2 (`|CreateWidget` "/Game/UI/WBP_VictoryMenu.WBP_VictoryMenu_C" _returnvalue))
    (`UserWidget.AddToViewport` _returnvalue_2 0)
    (`WidgetBlueprintLibrary.SetInputMode_UIOnlyEx` _returnvalue _returnvalue_2)
    (`ActorComponent.K2_DestroyComponent` (`self.RearBlocker`))
    ;[1 1 1] Victory Cutscene
    (`KismetSystemLibrary.Delay` 4.0)
    (`self.K2_DestroyActor` _asbp_player_phoenix)
    (else
      (`/Game/Blueprints/BP_PlayerPhoenix.BP_SendMessageToUI` _asbp_player_phoenix (`KismetTextLibrary.Conv_StringToText` "Chief Engineer: The gate is still offline, we need to activate those relays before we can escape.") true))))

(event `self.WarpGateAreaBox.OnComponentBeginOverlap`
  (params (OverlappedComponent :type "PrimitiveComponent Object Reference") (OtherActor :type "Actor Object Reference") (OtherComp :type "PrimitiveComponent Object Reference") (OtherBodyIndex :type Integer) (bFromSweep :type Boolean) (SweepResult :type "HitResult Structure (by ref)"))
  (bind _asbp_player_phoenix (cast `/Game/Blueprints/BP_PlayerPhoenix` OtherActor))
  (`/Game/Blueprints/BP_PlayerPhoenix.BP_SendMessageToUI` _asbp_player_phoenix "Navigator: We've reached the warp gate, captain. " true)
  (if (`self.bBossReadyToSpawn`)
    (`/Game/Blueprints/BP_PlayerPhoenix.BP_SendMessageToUI` _asbp_player_phoenix "Engineer: A large ship is creating a dampening field to disrupt the warp gate's power. We'll need to deal with that ship first before we can enter." true)
    (`/Game/Blueprints/BP_PlayerPhoenix.BP_SendMessageToUI` _asbp_player_phoenix "Defeat the dreadnought to restore the warp gate's power." false)
    (`self.SpawnBossEvent` _asbp_player_phoenix)))

(event `SpawnBossEvent`
  (params (InPlayerShip :type "JamShipBase Object Reference"))
  (`/Engine/EditorBlueprintResources/StandardMacros.DoOnce` false
    (:`Completed`
      (bind _returnvalue (`|SpawnActorFromClass` "/Game/Blueprints/BossFight/BP_BossShip.BP_BossShip_C" (`KismetMathLibrary.MakeTransform` (`SceneComponent.K2_GetComponentLocation` (`self.BossSpawn`)) (struct :`Yaw` -90.0)) "AlwaysSpawn" "OverrideRootScale" null null))
      (`/Engine/EditorBlueprintResources/StandardMacros.IsValid` _returnvalue :!label _label
        (:`Is Valid`
          (set `/Game/Blueprints/BossFight/BP_BossShip.WarpGateRef` self _returnvalue))
        (:`Is Not Valid`
          (`KismetSystemLibrary.Delay` 0.1)
          (goto _label))))))

(fn `ActivateWarpGate`
  (`PrimitiveComponent.SetCollisionEnabled` (`self.RearBlocker`) "QueryAndPhysics")
  (set `self.bBossReadyToSpawn` true))

(fn `BossDeath`
  (`MaterialInstanceDynamic.SetScalarParameterValue` (`self.DynamicMaterial`) "Glow" 20.0)
  (set `self.bGateActive` true)
  (`SceneComponent.SetVisibility` (`self.WarpFunnel`) true false)
  (`AudioComponent.FadeIn` (`self.SFXPortal`) 1.0 1.0 0.0 "Linear"))

(fn `UserConstructionScript`)