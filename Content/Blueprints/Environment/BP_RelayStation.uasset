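; Relay station that the player ship repairs by holding position inside its repair box, reporting progress through chief engineer comm messages.
; Overlap events with cross-resetting DoOnce nodes toggle repair state and red/green target planes, which Tick pulses by cycling visibility.
; The repair timer pauses outside the box without resetting.
; On completion, the planes are destroyed, the material glows, the station rotates and the game instance's quest check runs.
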(event `self.ReceiveBeginPlay`
  (bind _relaystationmesh (`self.RelayStationMesh`))
  (bind _returnvalue (`PrimitiveComponent.CreateDynamicMaterialInstance` _relaystationmesh 0 (`PrimitiveComponent.GetMaterial` _relaystationmesh 0) "None"))
  (bind _output_get (set `self.DynamicMaterial` _returnvalue))
  (`MaterialInstanceDynamic.SetScalarParameterValue` _output_get "Glow" 0.0)
  (bind _asbp_jam_game_instance (cast `/Game/Blueprints/BP_JamGameInstance` (`GameplayStatics.GetGameInstance`)))
  (bind _effectsvolpercent (`/Game/Blueprints/BP_JamGameInstance.EffectsVolPercent` _asbp_jam_game_instance))
  (`AudioComponent.SetVolumeMultiplier` (`self.SFXRepairedRelay`) _effectsvolpercent)
  (`AudioComponent.SetVolumeMultiplier` (`self.SFXRelayAmbience`) _effectsvolpercent))

(event `self.ReceiveTick`
  (params (DeltaSeconds :type "Float (single-precision)"))
  (if (`self.RepairComplete`)
    (`self.K2_AddActorLocalRotation` (`KismetMathLibrary.MakeRotator` (* DeltaSeconds 5.0)))
    (else
      (`self.PulseRepairAreaLines` DeltaSeconds)
      (`self.RepairInProgress` DeltaSeconds))))

(event `self.RelayStationRepairBox.OnComponentBeginOverlap`
  (params (OverlappedComponent :type "PrimitiveComponent Object Reference") (OtherActor :type "Actor Object Reference") (OtherComp :type "PrimitiveComponent Object Reference") (OtherBodyIndex :type Integer) (bFromSweep :type Boolean) (SweepResult :type "HitResult Structure (by ref)"))
  (if (not (`self.RepairComplete`))
    (bind _asbp_player_phoenix (cast `/Game/Blueprints/BP_PlayerPhoenix` OtherActor))
    (set `self.PlayerShipRef` _asbp_player_phoenix)
    (`/Engine/EditorBlueprintResources/StandardMacros.DoOnce` false :!label _label
      (:`Completed`
        (`/Game/Blueprints/BP_PlayerPhoenix.BP_SendMessageToUI` _asbp_player_phoenix "Chief Engineer: Hold position here, repairing the relay..." true)
        (set `self.RepairingRelay` true)
        (`self.ToggleRepairAreaLines` true)
        (goto _label_2 :!via `Reset`)))))

(event `self.RelayStationRepairBox.OnComponentEndOverlap`
  (params (OverlappedComponent :type "PrimitiveComponent Object Reference") (OtherActor :type "Actor Object Reference") (OtherComp :type "PrimitiveComponent Object Reference") (OtherBodyIndex :type Integer))
  (if (not (`self.RepairComplete`))
    (bind _asbp_player_phoenix (cast `/Game/Blueprints/BP_PlayerPhoenix` OtherActor))
    (`/Engine/EditorBlueprintResources/StandardMacros.DoOnce` false :!label _label_2
      (:`Completed`
        (`/Game/Blueprints/BP_PlayerPhoenix.BP_SendMessageToUI` _asbp_player_phoenix "Chief Engineer: Repairs are NOT complete. Please move closer to the relay." true)
        (set `self.RepairingRelay` false)
        (`self.ToggleRepairAreaLines` false)
        (goto _label :!via `Reset`)))))

(event `self.RelayStationArea.OnComponentBeginOverlap`
  (params (OverlappedComponent :type "PrimitiveComponent Object Reference") (OtherActor :type "Actor Object Reference") (OtherComp :type "PrimitiveComponent Object Reference") (OtherBodyIndex :type Integer) (bFromSweep :type Boolean) (SweepResult :type "HitResult Structure (by ref)"))
  (if (`self.RepairComplete`)
    (`AudioComponent.FadeIn` (`self.SFXRelayAmbience`) 3.0 1.0 0.0 "Linear")
    (else
      (bind _asbp_player_phoenix (cast `/Game/Blueprints/BP_PlayerPhoenix` OtherActor))
      (bind _output_get (set `self.PlayerShipRef` _asbp_player_phoenix))
      (`/Game/Blueprints/BP_PlayerPhoenix.BP_SendMessageToUI` _output_get "Chief Engineer: We've reached a relay station. Move the ship into position and I'll start the repairs." true))))

(event `self.RelayStationArea.OnComponentEndOverlap`
  (params (OverlappedComponent :type "PrimitiveComponent Object Reference") (OtherActor :type "Actor Object Reference") (OtherComp :type "PrimitiveComponent Object Reference") (OtherBodyIndex :type Integer))
  (cast `/Game/Blueprints/BP_PlayerPhoenix` OtherActor)
  (`AudioComponent.FadeOut` (`self.SFXRelayAmbience`) 3.0 0.0 "Linear"))

(fn `ActivateWarpGate`
  (`MaterialInstanceDynamic.SetScalarParameterValue` (`self.DynamicMaterial`) "Glow" 20.0)
  (set `self.bGateActive` true))

(fn `PulseRepairAreaLines`
  (params (InDelta :type "Float (double-precision)"))
  (if (not (`self.RepairComplete`))
    (bind _output_get (set `self.PulseTimer` (+ InDelta (`self.PulseTimer`))))
    (if (< _output_get (`self.PulseSpeed`))
      (`SceneComponent.SetVisibility` (`self.RepairAreaPlaneLarge`) true false)
      (`SceneComponent.SetVisibility` (`self.RepairAreaPlaneMid`) false false)
      (`SceneComponent.SetVisibility` (`self.RepairAreaPlaneSmall`) false false)
      (elif (< _output_get (* (`self.PulseSpeed`) 2.0))
        (`SceneComponent.SetVisibility` (`self.RepairAreaPlaneLarge`) false false)
        (`SceneComponent.SetVisibility` (`self.RepairAreaPlaneMid`) true false)
        (`SceneComponent.SetVisibility` (`self.RepairAreaPlaneSmall`) false false)
        (elif (< _output_get (* (`self.PulseSpeed`) 3.0))
          (`SceneComponent.SetVisibility` (`self.RepairAreaPlaneLarge`) false false)
          (`SceneComponent.SetVisibility` (`self.RepairAreaPlaneMid`) false false)
          (`SceneComponent.SetVisibility` (`self.RepairAreaPlaneSmall`) true false)
          (else
            (set `self.PulseTimer` 0.0)))))))

(fn `RepairCompleted`
  (bind _playershipref (`self.PlayerShipRef`))
  (`ActorComponent.K2_DestroyComponent` (`self.RepairAreaPlaneLarge`))
  (`ActorComponent.K2_DestroyComponent` (`self.RepairAreaPlaneMid`))
  (`ActorComponent.K2_DestroyComponent` (`self.RepairAreaPlaneSmall`))
  (`MaterialInstanceDynamic.SetScalarParameterValue` (`self.DynamicMaterial`) "Glow" 20.0)
  (`/Engine/EditorBlueprintResources/StandardMacros.IsValid` _playershipref
    (:`Is Valid`
      (`/Game/Blueprints/BP_PlayerPhoenix.BP_SendMessageToUI` _playershipref "Chief Engineer: This relay is operational, ready to move on, captain!" true)
      (bind _asbp_jam_game_instance (cast `/Game/Blueprints/BP_JamGameInstance` (`GameplayStatics.GetGameInstance`)))
      (`/Game/Blueprints/BP_JamGameInstance.CheckQuestRelayRepaired` _asbp_jam_game_instance self)
      (`AudioComponent.Play` (`self.SFXRepairedRelay`) 0.0))))

(fn `RepairInProgress`
  (params (A :type "Float (double-precision)"))
  (if (`self.RepairComplete`)
    _
    (elif (`self.RepairingRelay`)
      (bind _output_get (set `self.RepairTimer` (+ A (`self.RepairTimer`))))
      (if (> _output_get 10.0)
        (set `self.RepairComplete` true)
        (`self.RepairCompleted`)))))

(fn `ToggleRepairAreaLines`
  (params (Condition :type Boolean))
  (if Condition
    (`PrimitiveComponent.SetMaterial` (`self.RepairAreaPlaneLarge`) 0 "/Game/UI/Components/RelayTargetBoxGreen_M.RelayTargetBoxGreen_M")
    (`PrimitiveComponent.SetMaterial` (`self.RepairAreaPlaneMid`) 0 "/Game/UI/Components/RelayTargetBoxGreen_M.RelayTargetBoxGreen_M")
    (`PrimitiveComponent.SetMaterial` (`self.RepairAreaPlaneSmall`) 0 "/Game/UI/Components/RelayTargetBoxGreen_M.RelayTargetBoxGreen_M")
    (else
      (`PrimitiveComponent.SetMaterial` (`self.RepairAreaPlaneLarge`) 0 "/Game/UI/Components/RelayTargetBoxRed_M.RelayTargetBoxRed_M")
      (`PrimitiveComponent.SetMaterial` (`self.RepairAreaPlaneMid`) 0 "/Game/UI/Components/RelayTargetBoxRed_M.RelayTargetBoxRed_M")
      (`PrimitiveComponent.SetMaterial` (`self.RepairAreaPlaneSmall`) 0 "/Game/UI/Components/RelayTargetBoxRed_M.RelayTargetBoxRed_M"))))

(fn `UserConstructionScript`)