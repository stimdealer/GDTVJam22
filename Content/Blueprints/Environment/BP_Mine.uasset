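; Space mine hazard that homes in on the player ship and damages ships on contact.
; A proximity sphere toggles pursuit and material glow; Tick turns the mine and accelerates it toward the player, or applies velocity-opposing force when idle.
; An inner trigger sphere, tripped by any JamShipBase, damages overlapping ships, sets a plating glow, then destroys the mine after a short delay.
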(event `self.ReceiveTick`
  (params (DeltaSeconds :type "Float (single-precision)"))
  (bind _minemesh (`self.MineMesh`))
  (bind _playership (`self.PlayerShip`))
  (bind _returnvalue (`KismetMathLibrary.Normal` (- (`self.K2_GetActorLocation` _playership) (`self.K2_GetActorLocation`))))
  (if (`self.bPursuePlayer`)
    (`/Engine/EditorBlueprintResources/StandardMacros.IsValid` _playership
      (:`Is Valid`
        (`self.K2_SetActorRotation` self (`KismetMathLibrary.Conv_VectorToRotator` _returnvalue) false)
        (`PrimitiveComponent.AddForce` (`self.MineMesh`) (* _returnvalue 100.0) "None" true)))
    (else
      (`PrimitiveComponent.AddForce` _minemesh (* (`SceneComponent.GetComponentVelocity` _minemesh) -1.0) "None" true))))

(event `self.ReceiveBeginPlay`
  (bind _minemesh (`self.MineMesh`))
  (bind _returnvalue (`KismetMaterialLibrary.CreateDynamicMaterialInstance` (`StaticMesh.GetMaterial` (`StaticMeshComponent.StaticMesh` _minemesh) 0)))
  (bind _output_get (set `self.MineDynamicMaterial` _returnvalue))
  (`MaterialInstanceDynamic.SetScalarParameterValue` _output_get "Glow" 0.0)
  (`MaterialInstanceDynamic.SetScalarParameterValue` _output_get "Glow Plating" 0.0)
  (`PrimitiveComponent.SetMaterial` _minemesh 0 _output_get))

(event `self.ProximitySphere.OnComponentBeginOverlap`
  (params (OverlappedComponent :type "PrimitiveComponent Object Reference") (OtherActor :type "Actor Object Reference") (OtherComp :type "PrimitiveComponent Object Reference") (OtherBodyIndex :type Integer) (bFromSweep :type Boolean) (SweepResult :type "HitResult Structure (by ref)"))
  (bind _asbp_player_ship (cast `/Game/Blueprints/BP_PlayerShip` OtherActor))
  (set `self.PlayerShip` _asbp_player_ship)
  (`MaterialInstanceDynamic.SetScalarParameterValue` (`self.MineDynamicMaterial`) "Glow" 50.0)
  (set `self.bPursuePlayer` true))

(event `self.ProximitySphere.OnComponentEndOverlap`
  (params (OverlappedComponent :type "PrimitiveComponent Object Reference") (OtherActor :type "Actor Object Reference") (OtherComp :type "PrimitiveComponent Object Reference") (OtherBodyIndex :type Integer))
  (cast `/Game/Blueprints/BP_PlayerShip` OtherActor)
  (`MaterialInstanceDynamic.SetScalarParameterValue` (`self.MineDynamicMaterial`) "Glow" 0.0)
  (set `self.bPursuePlayer` false))

(event `self.TriggerSphere.OnComponentBeginOverlap`
  (params (OverlappedComponent :type "PrimitiveComponent Object Reference") (OtherActor :type "Actor Object Reference") (OtherComp :type "PrimitiveComponent Object Reference") (OtherBodyIndex :type Integer) (bFromSweep :type Boolean) (SweepResult :type "HitResult Structure (by ref)"))
  (cast `JamShipBase` OtherActor)
  (for _array_element (`PrimitiveComponent.GetOverlappingActors` (`self.TriggerSphere`) null)
    (bind _asjam_ship_base (cast `JamShipBase` _array_element))
    (`JamShipBase.ShipApplyDamage` _asjam_ship_base 60.0))
  (`MaterialInstanceDynamic.SetScalarParameterValue` (`self.MineDynamicMaterial`) "Plating Glow" 1.0)
  (`KismetSystemLibrary.Delay` 0.5)
  ;[1 1 1] Spawn Explosion VFX
  (`self.K2_DestroyActor` self))

(fn `UserConstructionScript`)