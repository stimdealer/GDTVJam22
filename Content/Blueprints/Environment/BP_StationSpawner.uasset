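; BP_StationSpawner is a slowly rotating station that spawns BP_NPCHunter enemies once the player's ship enters its trigger.
; On BeginPlay it sets a lifetime spawn cap scaled by the game instance's Difficulty.
; The trigger overlap stores the BP_PlayerPhoenix and permanently enables spawning.
; Tick then drives a timer that spawns hunters at SpawnPoint every few seconds, passing each the player ship reference, until the cap is reached.
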(event `self.ReceiveBeginPlay`
  (bind _asbp_jam_game_instance (cast `/Game/Blueprints/BP_JamGameInstance` (`GameplayStatics.GetGameInstance`)))
  (set `self.SpawnAmount` (+ (* (`/Game/Blueprints/BP_JamGameInstance.Difficulty` _asbp_jam_game_instance) 2) 3)))

(event `self.ReceiveTick`
  (params (DeltaSeconds :type "Float (single-precision)"))
  (`self.K2_AddActorWorldRotation` self (`KismetMathLibrary.MakeRotator` 0.0 0.0 (* DeltaSeconds 10.0)) false false)
  (`self.SpawnShips` DeltaSeconds))

(event `self.SpawnTrigger.OnComponentBeginOverlap`
  (params (OverlappedComponent :type "PrimitiveComponent Object Reference") (OtherActor :type "Actor Object Reference") (OtherComp :type "PrimitiveComponent Object Reference") (OtherBodyIndex :type Integer) (bFromSweep :type Boolean) (SweepResult :type "HitResult Structure (by ref)"))
  (bind _asbp_player_phoenix (cast `/Game/Blueprints/BP_PlayerPhoenix` OtherActor))
  (set `self.PlayerShip` _asbp_player_phoenix)
  (set `self.bSpawnShips` true))

(fn `SpawnShips`
  (params (A :type "Float (double-precision)"))
  (bind _playership (`self.PlayerShip`))
  (bind _output_get (set `self.SpawnTimer` (+ A (`self.SpawnTimer`))))
  (if (and (> _output_get 3.0) (`self.bSpawnShips`) (< (`self.SpawnCount`) (`self.SpawnAmount`)))
    (set `self.SpawnTimer` 0.0)
    (`/Engine/EditorBlueprintResources/StandardMacros.IsValid` _playership
      (:`Is Valid`
        (bind _returnvalue (`|SpawnActorFromClass` "/Game/Blueprints/BP_NPCHunter.BP_NPCHunter_C" (`KismetMathLibrary.MakeTransform` (`SceneComponent.K2_GetComponentLocation` (`self.SpawnPoint`))) "AdjustIfPossibleButAlwaysSpawn" "OverrideRootScale" null null))
        (`/Engine/EditorBlueprintResources/StandardMacros.IsValid` _returnvalue
          (:`Is Valid`
            (set `NPCShip.PlayerShipRef` _playership _returnvalue)
            (`/Engine/EditorBlueprintResources/StandardMacros.IncrementInt` (`self.SpawnCount`))))))))

(fn `UserConstructionScript`)