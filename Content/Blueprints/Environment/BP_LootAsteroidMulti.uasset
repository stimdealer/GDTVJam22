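; BP_LootAsteroidMulti is a lootable asteroid that carries both armor and fuel bonuses.
; Its construction script sets both bonuses, picks a random asteroid mesh and applies the multi glow material.
; Five meshes are wired, but RandomInteger(4) yields only 0 to 3, so SM_AsteroidE is never chosen.
; Tick calls the parent, then spins the mesh by a fixed local rotation each frame, independent of delta time.
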(event `self.ReceiveTick`
  (params (DeltaSeconds :type "Float (single-precision)"))
  (`parent.ReceiveTick` DeltaSeconds)
  (`SceneComponent.K2_AddLocalRotation` (`self.LootableMesh`) (struct :`Pitch` -0.5 :`Yaw` -0.5 :`Roll` 0.25) false false))

(fn `UserConstructionScript`
  (bind _lootablemesh (`self.LootableMesh`))
  (`parent.UserConstructionScript`)
  (set `self.ArmorBonus` 10.0)
  (set `self.FuelBonus` 10.0)
  (`|ExecutionSequence`
    (:`then_0`
      (switch `int` (`KismetMathLibrary.RandomInteger` 4)
        (:`0`
          (`StaticMeshComponent.SetStaticMesh` _lootablemesh "/Game/Models/Environment/Asteroids/SM_AsteroidA.SM_AsteroidA"))
        (:`1`
          (`StaticMeshComponent.SetStaticMesh` _lootablemesh "/Game/Models/Environment/Asteroids/SM_AsteroidB.SM_AsteroidB"))
        (:`2`
          (`StaticMeshComponent.SetStaticMesh` _lootablemesh "/Game/Models/Environment/Asteroids/SM_AsteroidC.SM_AsteroidC"))
        (:`3`
          (`StaticMeshComponent.SetStaticMesh` _lootablemesh "/Game/Models/Environment/Asteroids/SM_AsteroidD.SM_AsteroidD"))
        (:`4`
          (`StaticMeshComponent.SetStaticMesh` _lootablemesh "/Game/Models/Environment/Asteroids/SM_AsteroidE.SM_AsteroidE"))))
    (:`then_1`
      (`PrimitiveComponent.SetMaterial` (`self.LootableMesh`) 0 "/Game/Materials/MI_AsteroidsGlowMulti.MI_AsteroidsGlowMulti"))))