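; BP_LootableBase is a lootable pickup actor that grants a bonus to the player ship on contact.
; When its collision overlaps a PlayerShip, it passes its loot type and amount to the ship's ApplyLootableBonus.
; It then destroys its mesh, spawns an attached Niagara smoke puff, and destroys itself after a short delay.
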(event `self.Collision.OnComponentBeginOverlap`
  (params (OverlappedComponent :type "PrimitiveComponent Object Reference") (OtherActor :type "Actor Object Reference") (OtherComp :type "PrimitiveComponent Object Reference") (OtherBodyIndex :type Integer) (bFromSweep :type Boolean) (SweepResult :type "HitResult Structure (by ref)"))
  (bind _lootablemesh (`self.LootableMesh`))
  (bind _asplayer_ship (cast `PlayerShip` OtherActor))
  (`PlayerShip.ApplyLootableBonus` _asplayer_ship (`self.LootType`) (`self.LootAmount`))
  (`/Engine/EditorBlueprintResources/StandardMacros.IsValid` _lootablemesh
    (:`Is Valid`
      (`ActorComponent.K2_DestroyComponent` _lootablemesh))
    (:`Is Not Valid`
      _))
  (`NiagaraFunctionLibrary.SpawnSystemAttached` "/Game/VFX/NS_SmokePuff.NS_SmokePuff" (`self.DefaultSceneRoot`) "None" (0.0 0.0 0.0) (struct) "KeepRelativeOffset" true)
  (`KismetSystemLibrary.Delay` 1.0)
  (`self.K2_DestroyActor` self))

(fn `UserConstructionScript`)