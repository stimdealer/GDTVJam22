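; Proximity mine that homes in on the player ship and explodes on contact with ships, with damage set by game difficulty.
; The proximity sphere toggles pursuit and a dynamic-material glow as the player enters or leaves.
; Tick pushes the physics mesh toward the player, or damps its velocity when not pursuing.
; The trigger sphere damages overlapping ships immediately, then plays delayed explosion effects and destroys the mine.
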(event `self.ReceiveTick`
  (params (DeltaSeconds :type "Float (single-precision)"))
  (bind _minemesh (`self.MineMesh`))
  (bind _playership (`self.PlayerShip`))
  (bind _returnvalue (`KismetMathLibrary.Normal` (- (`self.K2_GetActorLocation` _playership) (`self.K2_GetActorLocation`))))
  (if (and (`self.bPursuePlayer`) (`SceneComponent.IsSimulatingPhysics` (`self.MineMesh`) "None"))
    (`/Engine/EditorBlueprintResources/StandardMacros.IsValid` _playership
      (:`Is Valid`
        (`self.K2_SetActorRotation` self (`KismetMathLibrary.Conv_VectorToRotator` _returnvalue) true)
        (`PrimitiveComponent.AddForce` (`self.MineMesh`) (* _returnvalue 250.0) "None" true)))
    (else
      (`PrimitiveComponent.AddForce` _minemesh (* (`SceneComponent.GetComponentVelocity` _minemesh) -1.0) "None" true))))

(event `self.ReceiveBeginPlay`
  (bind _minemesh (`self.MineMesh`))
  (bind _asbp_jam_game_instance (cast `/Game/Blueprints/BP_JamGameInstance` (`GameplayStatics.GetGameInstance`)))
  (`self.SetupMineDamage` (`/Game/Blueprints/BP_JamGameInstance.Difficulty` _asbp_jam_game_instance))
  (`AudioComponent.SetVolumeMultiplier` (`self.SFXExplode`) (`/Game/Blueprints/BP_JamGameInstance.EffectsVolPercent` _asbp_jam_game_instance))
  (bind _returnvalue (`KismetMaterialLibrary.CreateDynamicMaterialInstance` (`StaticMesh.GetMaterial` (`StaticMeshComponent.StaticMesh` _minemesh) 0)))
  (bind _output_get (set `self.MineDynamicMaterial` _returnvalue))
  (`MaterialInstanceDynamic.SetScalarParameterValue` _output_get "Glow" 0.0)
  (`MaterialInstanceDynamic.SetScalarParameterValue` _output_get "Glow Plating" 0.0)
  (`PrimitiveComponent.SetMaterial` _minemesh 0 _output_get))

(event `self.ProximitySphere.OnComponentBeginOverlap`
  (params (OverlappedComponent :type "PrimitiveComponent Object Reference") (OtherActor :type "Actor Object Reference") (OtherComp :type "PrimitiveComponent Object Reference") (OtherBodyIndex :type Integer) (bFromSweep :type Boolean) (SweepResult :type "HitResult Structure (by ref)"))
  (bind _asbp_player_phoenix (cast `/Game/Blueprints/BP_PlayerPhoenix` OtherActor))
  (set `self.PlayerShip` _asbp_player_phoenix)
  (`MaterialInstanceDynamic.SetScalarParameterValue` (`self.MineDynamicMaterial`) "Glow" 50.0)
  (set `self.bPursuePlayer` true))

(event `self.ProximitySphere.OnComponentEndOverlap`
  (params (OverlappedComponent :type "PrimitiveComponent Object Reference") (OtherActor :type "Actor Object Reference") (OtherComp :type "PrimitiveComponent Object Reference") (OtherBodyIndex :type Integer))
  (cast `/Game/Blueprints/BP_PlayerPhoenix` OtherActor)
  (`MaterialInstanceDynamic.SetScalarParameterValue` (`self.MineDynamicMaterial`) "Glow" 0.0)
  (set `self.bPursuePlayer` false))

(event `self.TriggerSphere.OnComponentBeginOverlap`
  (params (OverlappedComponent :type "PrimitiveComponent Object Reference") (OtherActor :type "Actor Object Reference") (OtherComp :type "PrimitiveComponent Object Reference") (OtherBodyIndex :type Integer) (bFromSweep :type Boolean) (SweepResult :type "HitResult Structure (by ref)"))
  (cast `JamShipBase` OtherActor)
  (for _array_element (`PrimitiveComponent.GetOverlappingActors` (`self.TriggerSphere`) null)
    (bind _asjam_ship_base (cast `JamShipBase` _array_element))
    (`JamShipBase.ShipApplyDamage` _asjam_ship_base (`self.Damage`)))
  (`MaterialInstanceDynamic.SetScalarParameterValue` (`self.MineDynamicMaterial`) "Plating Glow" 1.0)
  (`KismetSystemLibrary.Delay` 0.25)
  (`NiagaraFunctionLibrary.SpawnSystemAtLocation` "/Game/VFX/NS_GeneralExplosion.NS_GeneralExplosion" (`self.K2_GetActorLocation` self))
  (`AudioComponent.Play` (`self.SFXExplode`) 0.0)
  (`KismetSystemLibrary.Delay` 0.25)
  (`self.K2_DestroyActor` self))

(fn `SetupMineDamage`
  (params (InDifficulty :type Integer))
  (switch `int` InDifficulty
    (:`0`
      (set `self.Damage` 500.0))
    (:`1`
      (set `self.Damage` 1000.0))
    (:`2`
      (set `self.Damage` 1500.0))
    (:`3`
      (set `self.Damage` 2000.0))))

(fn `UserConstructionScript`)