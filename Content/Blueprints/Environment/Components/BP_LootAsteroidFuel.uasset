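; Fuel loot asteroid: a lootable environment object that sets loot type 2 with a random amount and tumbles in space.
; The construction script randomizes the mesh and per-axis spin and applies a glowing ore material.
; Its random index spans only four values, so the fifth mesh, SM_AsteroidE, is never chosen.
; Tick calls the parent, then applies the spin as a local rotation each frame, unscaled by delta time.
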(event `self.ReceiveTick`
  (params (DeltaSeconds :type "Float (single-precision)"))
  (`parent.ReceiveTick` DeltaSeconds)
  (`SceneComponent.K2_AddLocalRotation` (`self.LootableMesh`) (`KismetMathLibrary.MakeRotator` (`self.XRotation`) (`self.YRotation`) (`self.ZRotation`)) false false))

(fn `UserConstructionScript`
  (bind _lootablemesh (`self.LootableMesh`))
  (`parent.UserConstructionScript`)
  (set `self.LootType` 2)
  (set `self.LootAmount` (`KismetMathLibrary.RandomIntegerInRange` 10 30))
  (`|ExecutionSequence`
    (:`then_0`
      (switch `int` (`KismetMathLibrary.RandomInteger` 4)
        (:`0`
          (`StaticMeshComponent.SetStaticMesh` _lootablemesh "/Game/Models/Environment/Asteroids/SM_AsteroidA.SM_AsteroidA"))
        (:`1`
          (`StaticMeshComponent.SetStaticMesh` _lootablemesh "/Game/Models/Environment/Asteroids/SM_AsteroidB.SM_AsteroidB"))
        (:`2`
          (`StaticMeshComponent.SetStaticMesh` _lootablemesh "/Game/Models/Environment/Asteroids/SM_AsteroidC.SM_AsteroidC"))
        (:`3`
          (`StaticMeshComponent.SetStaticMesh` _lootablemesh "/Game/Models/Environment/Asteroids/SM_AsteroidD.SM_AsteroidD"))
        (:`4`
          (`StaticMeshComponent.SetStaticMesh` _lootablemesh "/Game/Models/Environment/Asteroids/SM_AsteroidE.SM_AsteroidE"))))
    (:`then_1`
      (`PrimitiveComponent.SetMaterial` (`self.LootableMesh`) 0 "/Game/Materials/MI_AsteroidsGlowOre.MI_AsteroidsGlowOre")
      (set `self.XRotation` (`KismetMathLibrary.RandomFloatInRange` -0.75 0.75))
      (set `self.YRotation` (`KismetMathLibrary.RandomFloatInRange` -0.75 0.75))
      (set `self.ZRotation` (`KismetMathLibrary.RandomFloatInRange` -0.75 0.75)))))