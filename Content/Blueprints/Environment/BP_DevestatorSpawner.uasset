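; BP_DevestatorSpawner is a one-shot encounter trigger that spawns an enemy Devestator with two Hunter escorts when BP_PlayerPhoenix enters its trigger sphere.
; The preview mesh is removed at BeginPlay, and the Devestator appears at the spawner's transform.
; Hunters get randomized positions, with X relative to the spawner but Y independent of it.
; Each NPC receives the player ship reference before the spawner destroys itself.
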(event `self.ReceiveBeginPlay`
  (`ActorComponent.K2_DestroyComponent` (`self.PreviewMesh`)))

(event `self.TriggerSphere.OnComponentBeginOverlap`
  (params (OverlappedComponent :type "PrimitiveComponent Object Reference") (OtherActor :type "Actor Object Reference") (OtherComp :type "PrimitiveComponent Object Reference") (OtherBodyIndex :type Integer) (bFromSweep :type Boolean) (SweepResult :type "HitResult Structure (by ref)"))
  (bind _returnvalue (`KismetMathLibrary.RandomFloatInRange` -5000.0 5000.0))
  (bind _returnvalue_2 (`self.GetTransform` self))
  (cast `/Game/Blueprints/BP_PlayerPhoenix` OtherActor)
  (bind _asjam_ship_base (cast `JamShipBase` OtherActor))
  (bind _returnvalue_3 (`|SpawnActorFromClass` "/Game/Blueprints/BP_NPCDevestator.BP_NPCDevestator_C" _returnvalue_2 "AdjustIfPossibleButAlwaysSpawn" "OverrideRootScale" null null))
  (set `NPCShip.PlayerShipRef` _asjam_ship_base _returnvalue_3)
  (for _ (range 2)
    (bind _returnvalue_4 (`|SpawnActorFromClass` "/Game/Blueprints/BP_NPCHunter.BP_NPCHunter_C" (`KismetMathLibrary.MakeTransform` (`KismetMathLibrary.MakeVector` (+ (.x (.location _returnvalue_2)) _returnvalue) (- 5000.0 _returnvalue))) "AdjustIfPossibleButAlwaysSpawn" "OverrideRootScale" null null))
    (set `NPCShip.PlayerShipRef` _asjam_ship_base _returnvalue_4))
  (`self.K2_DestroyActor` self))

(fn `UserConstructionScript`)