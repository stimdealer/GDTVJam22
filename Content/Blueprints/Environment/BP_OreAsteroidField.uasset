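; Ore asteroid field actor that scatters BP_LootAsteroidOre pickups around its location when play begins.
; The construction script previews a field with Amount mesh instances, placed using a seeded random stream and min/max spacing.
; BeginPlay destroys the previews and spawns asteroids with the same random placement formula on X and Y.
; The spawned count ignores Amount and shrinks as the game instance's Difficulty rises.
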(event `self.ReceiveBeginPlay`
  (bind _seed (`self.Seed`))
  (bind (_returnvalue_x _returnvalue_y) (`KismetMathLibrary.BreakVector` (+ (* (`KismetMathLibrary.RandomUnitVectorFromStream` _seed) (`KismetMathLibrary.RandomFloatInRangeFromStream` (`self.MinSpacing`) (`self.MaxSpacing`) _seed)) (`self.K2_GetActorLocation` self))))
  (`ActorComponent.K2_DestroyComponent` (`self.MeshPreviews`))
  (bind _asbp_jam_game_instance (cast `/Game/Blueprints/BP_JamGameInstance` (`GameplayStatics.GetGameInstance`)))
  (for _ (range 1 (+ (- 10 (* (`/Game/Blueprints/BP_JamGameInstance.Difficulty` _asbp_jam_game_instance) 2)) 1))
    (`|SpawnActorFromClass` "/Game/Blueprints/Environment/Components/BP_LootAsteroidOre.BP_LootAsteroidOre_C" (`KismetMathLibrary.MakeTransform` (`KismetMathLibrary.MakeVector` _returnvalue_x _returnvalue_y)) "AlwaysSpawn" "OverrideRootScale" null null)))

(fn `UserConstructionScript`
  (bind _seed (`self.Seed`))
  (bind (_returnvalue_x _returnvalue_y) (`KismetMathLibrary.BreakVector` (* (`KismetMathLibrary.RandomUnitVectorFromStream` _seed) (`KismetMathLibrary.RandomFloatInRangeFromStream` (`self.MinSpacing`) (`self.MaxSpacing`) _seed))))
  (for _ (range 1 (+ (`self.Amount`) 1))
    (`InstancedStaticMeshComponent.AddInstance` (`self.MeshPreviews`) (`KismetMathLibrary.MakeTransform` (`KismetMathLibrary.MakeVector` _returnvalue_x _returnvalue_y)) false)))