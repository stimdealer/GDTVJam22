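; Devestator enemy NPC ship that sets armor, shield, movement, firepower and loot from game-instance difficulty on BeginPlay.
; When targeted, it shows armor/shield bars and a turret marker that Tick spins and pulses along a curve.
; Death awards ore to the player, plays explosion effects and camera shakes, swaps in a wreck mesh, then destroys the actor.
; Turret firing audio is gated by paired DoOnce nodes, with effects volume from the game instance.
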(event `self.ReceiveBeginPlay`
  (`self.SpawnWeaponsVFX`)
  (`self.BP_SetupAudio`)
  (`self.SetupDevestatorStats`))

(event `self.ReceiveTick`
  (params (DeltaSeconds :type "Float (single-precision)"))
  (`self.AnimateTargetArrows` DeltaSeconds))

(event `self.ToggleTurretArrows`
  (params (IsActive :type Boolean))
  (set `self.bTargetTurrets` IsActive)
  (`self.BP_ToggleArrowsAndBars`))

(event `self.UpdateStats`
  (params (InArmorPercent :type "Float (single-precision)") (InShieldPercent :type "Float (single-precision)"))
  (bind _aswbp_enemy_bars (cast `/Game/UI/WBP_EnemyBars` (`WidgetComponent.GetWidget` (`self.StatusBars`))))
  (`/Game/UI/WBP_EnemyBars.SetStats` _aswbp_enemy_bars InArmorPercent InShieldPercent))

(event `self.ShipDeath`
  (bind _physicsroot (`self.PhysicsRoot`))
  (bind _asbp_player_phoenix (cast `/Game/Blueprints/BP_PlayerPhoenix` (`self.PlayerShipRef`)))
  (`PlayerShip.ApplyLootableBonus` _asbp_player_phoenix 3 (`self.OreLooted`))
  (`NiagaraFunctionLibrary.SpawnSystemAtLocation` "/Game/VFX/NS_DevestatorExplosion.NS_DevestatorExplosion" (`self.K2_GetActorLocation` self))
  (`PlayerController.ClientStartCameraShake` :`self` (`GameplayStatics.GetPlayerController` 0) :`Shake` "/Game/Blueprints/BP_CameraShake.BP_CameraShake_C" :`Scale` 0.25)
  (`AudioComponent.Play` (`self.SFXDeathExplode`) 0.0)
  (`AudioComponent.Stop` (`self.SFXTurret`))
  (`StaticMeshComponent.SetStaticMesh` _physicsroot "/Game/Models/Environment/Wrecks/CV2Wreck/SM_CV2_Wreck.SM_CV2_Wreck")
  (`PrimitiveComponent.SetSimulatePhysics` _physicsroot false)
  (`PrimitiveComponent.SetCollisionEnabled` _physicsroot "NoCollision")
  (`ActorComponent.K2_DestroyComponent` (`self.Sphere`))
  (`KismetSystemLibrary.Delay` 1.4)
  (`PlayerController.ClientStartCameraShake` :`self` (`GameplayStatics.GetPlayerController` 0) :`Shake` "/Game/Blueprints/BP_CameraShake.BP_CameraShake_C")
  (`KismetSystemLibrary.Delay` 1.6)
  (`self.K2_DestroyActor`))

(event `self.SFXTurretsFiring`
  (params (IsActive :type Boolean))
  (bind _sfxturret (`self.SFXTurret`))
  (if IsActive
    (`/Engine/EditorBlueprintResources/StandardMacros.DoOnce` false :!label _label
      (:`Completed`
        (`AudioComponent.Play` _sfxturret 0.0)
        (goto _label_2 :!via `Reset`)))
    (else
      (`/Engine/EditorBlueprintResources/StandardMacros.DoOnce` false :!label _label_2
        (:`Completed`
          (`AudioComponent.Stop` _sfxturret)
          (goto _label :!via `Reset`))))))

(fn `AnimateTargetArrows`
  (params (InDelta :type "Float (double-precision)"))
  (bind _targetturretmesh (`self.TargetTurretMesh`))
  (if (`SceneComponent.bVisible` _targetturretmesh)
    (`SceneComponent.K2_AddLocalRotation` _targetturretmesh (`KismetMathLibrary.MakeRotator` 0.0 0.0 (* InDelta 50.0)) false false)
    (bind _output_get (set `self.PulseTimer` (+ InDelta (`self.PulseTimer`))))
    (bind _returnvalue (/ (`CurveFloat.GetFloatValue` (`self.Curve`) _output_get) 4.0))
    (`SceneComponent.SetRelativeScale3D` _targetturretmesh (`KismetMathLibrary.MakeVector` _returnvalue _returnvalue _returnvalue))
    (if (> _output_get 1.0)
      (set `self.PulseTimer` 0.0))))

(fn `BP_SetupAudio`
  (bind _asbp_jam_game_instance (cast `/Game/Blueprints/BP_JamGameInstance` (`GameplayStatics.GetGameInstance`)))
  (bind _effectsvolpercent (`/Game/Blueprints/BP_JamGameInstance.EffectsVolPercent` _asbp_jam_game_instance))
  (`AudioComponent.SetVolumeMultiplier` (`self.SFXDeathExplode`) _effectsvolpercent)
  (`AudioComponent.SetVolumeMultiplier` (`self.SFXTurret`) _effectsvolpercent))

(fn `BP_StartPhysics`
  (`PrimitiveComponent.SetSimulatePhysics` (`self.PhysicsRoot`) true)
  (set `self.PendingStartPhysics` false))

(fn `BP_ToggleArrowsAndBars`
  (bind _targetturretmesh (`self.TargetTurretMesh`))
  (bind _btargetturrets (`self.bTargetTurrets`))
  (bind _statusbars (`self.StatusBars`))
  (`|ExecutionSequence`
    (:`then_0`
      (`/Engine/EditorBlueprintResources/StandardMacros.IsValid` _targetturretmesh
        (:`Is Valid`
          (`SceneComponent.SetVisibility` _targetturretmesh _btargetturrets true))))
    (:`then_1`
      (`/Engine/EditorBlueprintResources/StandardMacros.IsValid` _statusbars
        (:`Is Valid`
          (`SceneComponent.SetVisibility` _statusbars _btargetturrets true))))))

(fn `SetupDevestatorStats`
  (set `self.bShieldEnabled` true)
  (bind _asbp_jam_game_instance (cast `/Game/Blueprints/BP_JamGameInstance` (`GameplayStatics.GetGameInstance`)))
  (switch `int` (`/Game/Blueprints/BP_JamGameInstance.Difficulty` _asbp_jam_game_instance)
    (:`0`
      (bind _output_get (set `self.MaxArmor` 500.0))
      (set `self.CurrentArmor` _output_get)
      (bind _output_get_2 (set `self.MaxShield` 200.0))
      (set `self.CurrentShield` _output_get_2)
      (set `self.ShieldRegenAmount` 10.0)
      (set `self.MaxSpeed` 200.0)
      (set `self.TurnSpeed` 20.0)
      (set `self.ForwardFirepower` 50.0)
      (set `self.OreLooted` 20)
      (set `self.ForwardRange` 7000.0))
    (:`1`
      (bind _output_get_3 (set `self.MaxArmor` 500.0))
      (set `self.CurrentArmor` _output_get_3)
      (bind _output_get_4 (set `self.MaxShield` 200.0))
      (set `self.CurrentShield` _output_get_4)
      (set `self.ShieldRegenAmount` 25.0)
      (set `self.MaxSpeed` 200.0)
      (set `self.TurnSpeed` 20.0)
      (set `self.ForwardFirepower` 50.0)
      (set `self.OreLooted` 20)
      (set `self.ForwardRange` 8000.0))
    (:`2`
      (bind _output_get_5 (set `self.MaxArmor` 700.0))
      (set `self.CurrentArmor` _output_get_5)
      (bind _output_get_6 (set `self.MaxShield` 250.0))
      (set `self.CurrentShield` _output_get_6)
      (set `self.ShieldRegenAmount` 25.0)
      (set `self.MaxSpeed` 250.0)
      (set `self.TurnSpeed` 30.0)
      (set `self.ForwardFirepower` 60.0)
      (set `self.OreLooted` 15)
      (set `self.ForwardRange` 8000.0))
    (:`3`
      (bind _output_get_7 (set `self.MaxArmor` 700.0))
      (set `self.CurrentArmor` _output_get_7)
      (bind _output_get_8 (set `self.MaxShield` 250.0))
      (set `self.CurrentShield` _output_get_8)
      (set `self.ShieldRegenAmount` 25.0)
      (set `self.MaxSpeed` 250.0)
      (set `self.TurnSpeed` 30.0)
      (set `self.ForwardFirepower` 60.0)
      (set `self.OreLooted` 15)
      (set `self.ForwardRange` 8000.0))))

(fn `UserConstructionScript`)