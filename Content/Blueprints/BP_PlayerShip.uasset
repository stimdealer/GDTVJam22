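; Player ship Blueprint that takes click-to-set-destination input and relays ship status to the HUD.
; On BeginPlay it adds its two turrets to the Turrets array.
; Left click runs a complex cursor trace against a single object type and stores the hit location as Destination; movement is not handled in this graph.
; Two events pass armor and fuel percentages and text messages to PlayerHUD when it is valid.
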(event `self.ReceiveBeginPlay`
  (bind _turrets (`self.Turrets`))
  (`KismetArrayLibrary.Array_Add` _turrets (`self.Turret_01`))
  (`KismetArrayLibrary.Array_Add` _turrets (`self.Turret_02`)))

(event `Key|LeftMouseButton`
  (params (Key :type "Key Structure"))
  (bind (_bblockinghit _binitialoverlap _time _distance _location) (`GameplayStatics.BreakHitResult` (`PlayerController.GetHitResultUnderCursorForObjects` (`GameplayStatics.GetPlayerController` 0) (`|MakeArray` "ObjectTypeQuery7" :!type "EObjectTypeQuery Enum") true)))
  (:`Pressed`
    (if _bblockinghit
      (set `self.Destination` _location))))

(event `self.SendArmorFuelToUI`
  (params (InArmorPercent :type "Float (single-precision)") (InFuelPercent :type "Float (single-precision)"))
  (bind _playerhud (`self.PlayerHUD`))
  (`/Engine/EditorBlueprintResources/StandardMacros.IsValid` _playerhud
    (:`Is Valid`
      (`ProgressBar.SetPercent` (`/Game/UI/WBP_MainGameHUD.BarArmor` _playerhud) InArmorPercent)
      (`ProgressBar.SetPercent` (`/Game/UI/WBP_MainGameHUD.BarFuel` _playerhud) InFuelPercent))))

(event `self.SendMessageToUI`
  (params (InMessage :type "Text (by ref)"))
  (bind _playerhud (`self.PlayerHUD`))
  (`/Engine/EditorBlueprintResources/StandardMacros.IsValid` _playerhud
    (:`Is Valid`
      (`/Game/UI/WBP_MainGameHUD.SetMessage` _playerhud InMessage))))

(fn `UserConstructionScript`)