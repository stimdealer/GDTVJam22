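; NPC hunter ship Blueprint that handles the ship's turret setup, targeting indicators, status bars, audio and death.
; BeginPlay registers its turret, spawns weapon VFX and sets up audio, with SFX volume read from the game instance.
; Tick spins visible turret and broadside arrows in opposite directions, pulsing the turret one by curve.
; Death plays explosion effects, swaps in a wreck mesh, disables physics and collision, then destroys the actor after a delay.
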(event `self.ReceiveBeginPlay`
  (`KismetArrayLibrary.Array_Add` (`self.Turrets`) (`self.Turret_1`))
  (`self.SpawnWeaponsVFX`)
  (`self.BP_SetupAudio`))

(event `self.ReceiveTick`
  (params (DeltaSeconds :type "Float (single-precision)"))
  (`self.AnimateTargetArrows` DeltaSeconds))

(event `self.ToggleArrows`
  (params (IsVisible :type Boolean))
  (`self.BP_ToggleArrowsAndBars` false))

(event `self.UpdateStats`
  (params (InArmorPercent :type "Float (single-precision)"))
  (bind _aswbp_enemy_bars (cast `/Game/UI/WBP_EnemyBars` (`WidgetComponent.GetWidget` (`self.StatusBars`))))
  (`/Game/UI/WBP_EnemyBars.SetStats` _aswbp_enemy_bars InArmorPercent))

(event `self.ShipDeath`
  (bind _physicsroot (`self.PhysicsRoot`))
  (`NiagaraFunctionLibrary.SpawnSystemAtLocation` "/Game/VFX/NS_ShipExplosion.NS_ShipExplosion" (`self.K2_GetActorLocation` self))
  (`AudioComponent.Play` (`self.SFXDeathExplode`) 0.0)
  (`StaticMeshComponent.SetStaticMesh` _physicsroot "/Game/Models/Environment/Wrecks/CV2Wreck/SM_CV2_Wreck.SM_CV2_Wreck")
  (`PrimitiveComponent.SetSimulatePhysics` _physicsroot false)
  (`PrimitiveComponent.SetCollisionEnabled` _physicsroot "NoCollision")
  (`ActorComponent.K2_DestroyComponent` (`self.Sphere`))
  (`KismetSystemLibrary.Delay` 3.0)
  (`self.K2_DestroyActor`))

(event `self.SFXTurretsFiring`
  (params (IsActive :type Boolean))
  (bind _sfxturret (`self.SFXTurret`))
  (if IsActive
    (`/Engine/EditorBlueprintResources/StandardMacros.DoOnce` false :!label _label
      (:`Completed`
        (`AudioComponent.Play` _sfxturret 0.0)
        (goto _label_2 :!via `Reset`)))
    (else
      (`/Engine/EditorBlueprintResources/StandardMacros.DoOnce` false :!label _label_2
        (:`Completed`
          (`AudioComponent.Stop` _sfxturret)
          (goto _label :!via `Reset`))))))

(fn `AnimateTargetArrows`
  (params (InDelta :type "Float (double-precision)"))
  (bind _returnvalue (* InDelta 50.0))
  (bind _targetturretmesh (`self.TargetTurretMesh`))
  (bind _targetbroadsidemesh (`self.TargetBroadsideMesh`))
  (`|ExecutionSequence`
    (:`then_0`
      (if (`SceneComponent.bVisible` _targetturretmesh)
        (`SceneComponent.K2_AddLocalRotation` _targetturretmesh (`KismetMathLibrary.MakeRotator` 0.0 0.0 _returnvalue) false false)
        (bind _output_get (set `self.PulseTimer` (+ InDelta (`self.PulseTimer`))))
        (bind _returnvalue_2 (`CurveFloat.GetFloatValue` (`self.Curve`) _output_get))
        (`SceneComponent.SetRelativeScale3D` _targetturretmesh (`KismetMathLibrary.MakeVector` _returnvalue_2 _returnvalue_2 _returnvalue_2))
        (if (> _output_get 1.0)
          (set `self.PulseTimer` 0.0))))
    (:`then_1`
      (if (`SceneComponent.bVisible` _targetbroadsidemesh)
        (`SceneComponent.K2_AddLocalRotation` _targetbroadsidemesh (`KismetMathLibrary.MakeRotator` 0.0 0.0 (* _returnvalue -1.0)) false false)))))

(fn `BP_SetupAudio`
  (bind _asbp_jam_game_instance (cast `/Game/Blueprints/BP_JamGameInstance` (`GameplayStatics.GetGameInstance`)))
  (bind _effectsvolpercent (`/Game/Blueprints/BP_JamGameInstance.EffectsVolPercent` _asbp_jam_game_instance))
  (`AudioComponent.SetVolumeMultiplier` (`self.SFXDeathExplode`) _effectsvolpercent)
  (`AudioComponent.SetVolumeMultiplier` (`self.SFXTurret`) _effectsvolpercent))

(fn `BP_StartPhysics`
  (`PrimitiveComponent.SetSimulatePhysics` (`self.PhysicsRoot`) true)
  (set `self.PendingStartPhysics` false))

(fn `BP_ToggleArrowsAndBars`
  (params (bTurrets :type Boolean) (bBroadsides :type Boolean))
  (bind _targetturretmesh (`self.TargetTurretMesh`))
  (bind _statusbars (`self.StatusBars`))
  (bind _targetbroadsidemesh (`self.TargetBroadsideMesh`))
  (`|ExecutionSequence`
    (:`then_0`
      (`/Engine/EditorBlueprintResources/StandardMacros.IsValid` _targetturretmesh
        (:`Is Valid`
          (`SceneComponent.SetVisibility` _targetturretmesh bTurrets true))))
    (:`then_1`
      (`/Engine/EditorBlueprintResources/StandardMacros.IsValid` _targetbroadsidemesh
        (:`Is Valid`
          (`SceneComponent.SetVisibility` _targetbroadsidemesh bBroadsides true))))
    (:`then_2`
      (`/Engine/EditorBlueprintResources/StandardMacros.IsValid` _statusbars
        (:`Is Valid`
          (`SceneComponent.SetVisibility` _statusbars (or bTurrets bBroadsides) true))))))

(fn `UserConstructionScript`)