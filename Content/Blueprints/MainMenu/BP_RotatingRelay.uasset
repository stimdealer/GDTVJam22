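; BP_RotatingRelay is a main menu actor that shows a relay mesh slowly spinning with an animated glow.
; BeginPlay creates a dynamic material instance from the Relay component's first material.
; Tick rolls the actor at a frame-rate independent speed and calls Play on the GlowVar timeline, whose scaled Glow track drives the material's Glow scalar parameter.
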(event `self.ReceiveBeginPlay`
  (bind _relay (`self.Relay`))
  (bind _returnvalue (`PrimitiveComponent.CreateDynamicMaterialInstance` _relay 0 (`PrimitiveComponent.GetMaterial` _relay 0) "None"))
  (set `self.DynamicMaterial` _returnvalue))

(event `self.ReceiveTick`
  (params (DeltaSeconds :type "Float (single-precision)"))
  (`self.K2_AddActorLocalRotation` (`KismetMathLibrary.MakeRotator` (* DeltaSeconds 5.0)))
  (bind (_direction _glow) (`Timeline|GlowVar`)
    (:`Update`
      (`MaterialInstanceDynamic.SetScalarParameterValue` (`self.DynamicMaterial`) "Glow" (* _glow 20.0)))))

(fn `UserConstructionScript`)