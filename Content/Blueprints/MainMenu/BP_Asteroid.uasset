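; Main menu asteroid actor that tumbles continuously as set dressing.
; The construction script picks a random rotation rate for each axis between MinRot and MaxRot.
; Tick applies those rates, scaled by delta time, as local rotation on the Asteroid component for a frame-rate independent spin.
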(event `self.ReceiveTick`
  (params (DeltaSeconds :type "Float (single-precision)"))
  (`SceneComponent.K2_AddLocalRotation` (`self.Asteroid`) (`KismetMathLibrary.MakeRotator` (* DeltaSeconds (`self.XRot`)) (* DeltaSeconds (`self.YRot`)) (* DeltaSeconds (`self.ZRot`))) false false))

(fn `UserConstructionScript`
  (bind _minrot (`self.MinRot`))
  (bind _maxrot (`self.MaxRot`))
  (set `self.XRot` (`KismetMathLibrary.RandomFloatInRange` _minrot _maxrot))
  (set `self.YRot` (`KismetMathLibrary.RandomFloatInRange` _minrot _maxrot))
  (set `self.ZRot` (`KismetMathLibrary.RandomFloatInRange` _minrot _maxrot)))