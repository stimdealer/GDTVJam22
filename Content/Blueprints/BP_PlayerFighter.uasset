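; Player fighter Blueprint that handles the gatling gun sound effect for forward firing.
; On BeginPlay it sets the GatlingSFX volume from the effects volume stored in BP_JamGameInstance.
; SFXForwardFiring uses two DoOnce gates that reset each other, so the sound plays or stops only when the firing state changes, not on every call.
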(event `self.ReceiveBeginPlay`
  (bind _asbp_jam_game_instance (cast `/Game/Blueprints/BP_JamGameInstance` (`GameplayStatics.GetGameInstance`)))
  (`AudioComponent.SetVolumeMultiplier` (`self.GatlingSFX`) (`/Game/Blueprints/BP_JamGameInstance.EffectsVolPercent` _asbp_jam_game_instance)))

(event `self.SFXForwardFiring`
  (params (IsActive :type Boolean))
  (bind _gatlingsfx (`self.GatlingSFX`))
  (if IsActive
    (`/Engine/EditorBlueprintResources/StandardMacros.DoOnce` false :!label _label
      (:`Completed`
        (`AudioComponent.Play` _gatlingsfx 0.0)
        (goto _label_2 :!via `Reset`)))
    (else
      (`/Engine/EditorBlueprintResources/StandardMacros.DoOnce` false :!label _label_2
        (:`Completed`
          (`AudioComponent.Stop` _gatlingsfx)
          (goto _label :!via `Reset`))))))

(fn `UserConstructionScript`)